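; A physics conveyor belt that appears to move objects along its surface using collision friction and a jittering helper component.
; Tick alternates between setting zero friction while starting a move of MovementHelper backwards along X by a speed-based offset, and switching to rubber friction while snapping it back to origin without teleporting.
; The construction script locks actor scale to one and sizes the helper and visuals from Size as a thin slab.
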(event `self.ReceiveTick`
  (params (DeltaSeconds :type "Float (single-precision)"))
  (`SceneComponent.K2_SetRelativeLocation` (`self.Movement Helper`) (0.0 0.0 0.0) false false)
  (`/Engine/EditorBlueprintResources/StandardMacros.FlipFlop`
    (:`A`
      (`PrimitiveComponent.SetPhysMaterialOverride` (`self.Conveyor Collision Object`) "/Game/Afterlife/Maps/Conveyor/ZeroFriction.ZeroFriction")
      (`KismetSystemLibrary.MoveComponentTo` (`self.Movement Helper`) (`KismetMathLibrary.MakeVector` (* (`self.Speed cm/s`) -1.0)) :!label _label))
    (:`B`
      (`PrimitiveComponent.SetPhysMaterialOverride` (`self.Conveyor Collision Object`) "/Engine/EngineMaterials/PhysMat_Rubber.PhysMat_Rubber")
      (`SceneComponent.K2_SetRelativeLocation` (`self.Movement Helper`) (0.0 0.0 0.0) false false)
      (`|ExecutionSequence`
        (:`then_0`
          (goto _label :!via `Return`))
        (:`then_1`
          (goto _label :!via `Stop`))))))

(fn `UserConstructionScript`
  (bind (_size_x _size_y) (`KismetMathLibrary.BreakVector2D` (`self.Size`)))
  (`self.SetActorScale3D` (1.0 1.0 1.0))
  (`SceneComponent.SetRelativeScale3D` (`self.Movement Helper`) (`KismetMathLibrary.MakeVector` _size_x _size_y 0.03))
  (`SceneComponent.SetRelativeScale3D` (`self.Visuals`) (`KismetMathLibrary.MakeVector` _size_x _size_y 0.03)))
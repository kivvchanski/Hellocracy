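; BP_LongStaminaBuff is an item effect that temporarily raises the user's stamina regeneration rate.
; Use calls the parent, then adds FloatParameter to the regen rate on the user's StaminaComponent.
; Stop calls the parent, then subtracts the same parameter from the current rate, undoing the boost additively rather than restoring a saved value.
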(fn `Stop`
  (bind _staminacomponent (`MainCharacter.StaminaComponent` (`self.User`)))
  (`parent.Stop`)
  (bind _returnvalue (`StaminaComponent.GetStaminaRegenRate` _staminacomponent))
  (`StaminaComponent.SetStaminaRegenRate` _staminacomponent (- _returnvalue (`self.FloatParameter`))))

(fn `Use`
  (params (User :type "/Game/Afterlife/Framework/Player/BP_MainCharacter Object Reference"))
  (bind _staminacomponent (`MainCharacter.StaminaComponent` (`self.User`)))
  (`parent.Use` User)
  (bind _returnvalue (`StaminaComponent.GetStaminaRegenRate` _staminacomponent))
  (`StaminaComponent.SetStaminaRegenRate` _staminacomponent (+ _returnvalue (`self.FloatParameter`))))
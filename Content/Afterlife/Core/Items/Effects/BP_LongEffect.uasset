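; BP_LongEffect is an item effect that stays active on its user for a set duration.
; Use stops any effect already stored under the same name, appends "_1" to its own name, registers itself in the user's Effects map and requests a timer for its Length through AddEffectTimer.
; Stop removes the entry from that map, and both functions print debug messages.
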(fn `Stop`
  (`BlueprintMapLibrary.Map_Remove` (`/Game/Afterlife/Framework/Player/BP_MainCharacter.Effects` (`self.User`)) (`self.EffectName`))
  (`KismetSystemLibrary.PrintString` null (`KismetStringLibrary.Concat_StrStr` "STOP EFFECT" " \n" (`self.EffectName`)) true true (struct :`R` 1.0 :`G` 0.011409 :`B` 4.8e-05 :`A` 1.0) 6.0))

(fn `Use`
  (params (User :type "/Game/Afterlife/Framework/Player/BP_MainCharacter Object Reference"))
  (bind _effects (`/Game/Afterlife/Framework/Player/BP_MainCharacter.Effects` User))
  (bind (_value _returnvalue) (`BlueprintMapLibrary.Map_Find` _effects (`self.EffectName`)))
  (set `self.User` User)
  (if _returnvalue
    (`self.Stop` _value)
    (set `self.EffectName` (`KismetStringLibrary.Concat_StrStr` (`self.EffectName`) "_1")))
  (`BlueprintMapLibrary.Map_Add` _effects (`self.EffectName`) self)
  (`KismetSystemLibrary.PrintString` null (`KismetStringLibrary.Concat_StrStr` "START EFFECT" " \n" (`self.EffectName`)) true true (struct :`R` 1.0 :`G` 0.011409 :`B` 4.8e-05 :`A` 1.0) 6.0)
  (`/Game/Afterlife/Framework/Player/BP_MainCharacter.AddEffectTimer` (`self.User`) (`self.EffectName`) (`self.Length`)))
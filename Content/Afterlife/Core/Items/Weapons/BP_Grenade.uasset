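; BP_Grenade is a throwable weapon item that hides its own mesh on begin play.
; Its main action spawns a BP_GrenadeTile at the user's scene transform, passes it damage, mesh, radius, fuse, push force and thrower, then launches it along the camera's forward vector.
; A DoOnce gate resets after the grenade delay, limiting throw rate.
; Count and reload logic exists but is disconnected.
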(event `self.ReceiveBeginPlay`
  (`parent.ReceiveBeginPlay`)
  (`SceneComponent.SetVisibility` (`self.GrenadeMesh`) false false))

(event `self.StartMainAction`
  (bind _userref (`self.UserRef`))
  (`/Engine/EditorBlueprintResources/StandardMacros.DoOnce` false :!label _label
    (:`Completed`
      (`/Game/Afterlife/Framework/Player/BP_MainCharacter.OnPickUpUpdate` (`self.UserRef`))
      (bind _returnvalue (`|SpawnActorFromClass` "/Game/Afterlife/Core/Items/Weapons/BP_GrenadeTile.BP_GrenadeTile_C" (`SceneComponent.K2_GetComponentToWorld` (`/Game/Afterlife/Framework/Player/BP_MainCharacter.Scene` (`self.UserRef`))) "Undefined" "MultiplyWithRoot" null null))
      (`/Game/Afterlife/Core/Items/Weapons/BP_GrenadeTile.Init` _returnvalue (`self.Damage`) (`StaticMeshComponent.StaticMesh` (`self.GrenadeMesh`)) (`self.Radius`) (`self.GrenadeDelay`) (`self.PushingForce`) _userref)
      (`/Game/Afterlife/Core/Items/Weapons/BP_GrenadeTile.Launch` _returnvalue (* (`SceneComponent.GetForwardVector` (`MainCharacter.FollowCamera` _userref)) (`self.ThrowPower`)))
      (`KismetSystemLibrary.Delay` (`self.GrenadeDelay`))
      (goto _label :!via `Reset`))))

(fn `UserConstructionScript`
  (`parent.UserConstructionScript`))
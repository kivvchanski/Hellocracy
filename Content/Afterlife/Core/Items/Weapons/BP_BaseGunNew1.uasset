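; Base gun item for the player: hitscan shooting, inventory-backed ammo and reloading, with animation events meant for child overrides.
; Each shot deprojects randomized screen-center points for per-bullet spread traces, damages BPI_Damagable actors and plays effects, with blood on Enemy-tagged hits.
; DoOnce plus Delay limits fire rate, while a looping timer repeats shots for bursts.
; Equip and reload draw ammo from inventory slots; unequip returns it; firing reports AI noise.
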(event `self.OnEquip`
  (bind _userref (`self.UserRef`))
  (bind _emitterpoint (`/Game/Afterlife/Framework/Player/BP_MainCharacter.EmitterPoint` _userref))
  ; Comment
  (`parent.OnEquip`)
  (for _array_element (`InventoryComponent.InventorySlots` (`MainCharacter.GetInventoryComponent` _userref))
    (bind (_item _quantity) (break `InventorySlot` _array_element))
    (if (== (break `Item` _item) (`self.AmmoType`))
      (set `self.InventotyAmmo` (+ (`self.InventotyAmmo`) _quantity))
      (set `self.AmmoInfo` (`.Item` (break `InventorySlot` _array_element)))))
  (`self.UpdateAmmoCount`)
  (`/Game/Afterlife/Framework/Player/BP_MainCharacter.ChangeAmmoCount` (`self.UserRef`) 0 (`self.InventotyAmmo`))
  (`/Game/Afterlife/Core/BattleSystem/BPI_Reloadable.Reload` (`self.MaxAmmo`))
  (`/Game/Afterlife/Framework/Player/BP_MainCharacter.ChangeWeapon` _userref false)
  (set `self.Emitter Point` _emitterpoint)
  (`SceneComponent.K2_AttachToComponent` (`self.FireEffectEmmiter`) _emitterpoint "None" "SnapToTarget" "SnapToTarget" "SnapToTarget" true)
  (`/Game/Afterlife/Framework/Player/BP_MainCharacter.SetVisibleAmmo` (`self.UserRef`)))

(event `self.OnUnEquip`
  (`InventoryComponent.AddItem` (`MainCharacter.GetInventoryComponent` (`self.UserRef`)) (`self.AmmoInfo`) (`self.CurrentAmmo`))
  (`self.UpdateAmmoCount`))

(event `self.ReceiveBeginPlay`
  (set `self.CanShoot` true))

(event `self.StartMainAction`
  (bind _returnvalue (`GameplayStatics.GetPlayerController` 0))
  (bind _userref (`self.UserRef`))
  (bind _tempfirerate (`self.TempFireRate`))
  (bind _returnvalue_2 (* (`self.FireDistance(m)`) 100.0))
  (if (`self.CanShoot`)
    (if (`self.IsBursting`)
      (set `self.TempFireRate` (`self.FireRateBurst`))
      (else
        (set `self.TempFireRate` (`self.FireRateDelay`))))
    (`/Engine/EditorBlueprintResources/StandardMacros.DoOnce` false :!label _label
      (:`Completed`
        (if (> (`self.CurrentAmmo`) 0)
          (`/Engine/EditorBlueprintResources/StandardMacros.DecrementInt` (`self.CurrentAmmo`)
            (:`  `
              (`/Game/Afterlife/Framework/Player/BP_MainCharacter.ChangeAmmoCount` (`self.UserRef`) (`self.CurrentAmmo`) (`self.InventotyAmmo`))
              (`self.FireAnim`)
              (for _ (range 1 (+ (`self.BulletsPerShot`) 1))
                (bind _returnvalue_3 (`WidgetLayoutLibrary.GetPlayerScreenWidgetGeometry` _returnvalue))
                (bind (_returnvalue_x _returnvalue_y) (`KismetMathLibrary.BreakVector2D` (`SlateBlueprintLibrary.GetAbsoluteSize` _returnvalue_3)))
                (bind _returnvalue_4 (/ _returnvalue_y 2.0))
                (bind _returnvalue_5 (* _returnvalue_4 (/ (* (`self.SpreadIntensityBase`) (`self.SpreadMultiplyer`)) 100.0)))
                (bind _returnvalue_6 (* _returnvalue_5 -1.0))
                (bind (_worldposition _worlddirection) (`GameplayStatics.DeprojectScreenToWorld` _returnvalue (`KismetMathLibrary.MakeVector2D` (+ (/ _returnvalue_x 2.0) (`KismetMathLibrary.RandomFloatInRange` _returnvalue_6 _returnvalue_5)) (+ _returnvalue_4 (`KismetMathLibrary.RandomFloatInRange` _returnvalue_6 _returnvalue_5)))))
                (bind _outhit (`KismetSystemLibrary.LineTraceSingle` (`SceneComponent.K2_GetComponentLocation` (`/Game/Afterlife/Framework/Player/BP_MainCharacter.ViewPoint` (`self.UserRef`))) (+ _worldposition (`KismetMathLibrary.MakeVector` (* (.x _worlddirection) _returnvalue_2) (* (.y _worlddirection) _returnvalue_2) (* (.z _worlddirection) _returnvalue_2))) "TraceTypeQuery1"))
                (`GameplayStatics.PlaySound2D` (`self.ShotSound`) 1.0 1.0 0.0 null null)
                (bind (_bblockinghit _binitialoverlap _time _distance _location _impactpoint _normal _impactnormal _physmat _hitactor) (`GameplayStatics.BreakHitResult` _outhit))
                (if (`self.ActorHasTag` _hitactor "Enemy")
                  (set `self.HitEffect` "/Game/Afterlife/VFX/Packs/Realistic_Starter_VFX_Pack_Vol2/Particles/Blood/P_Blood_Splat_Cone.P_Blood_Splat_Cone")
                  (else
                    (set `self.HitEffect` "/Game/Afterlife/VFX/Packs/Realistic_Starter_VFX_Pack_Vol2/Particles/Hit/P_Asphalt.P_Asphalt")))
                (`self.HiEffect` _impactpoint)
                (if (`KismetSystemLibrary.DoesImplementInterface` _hitactor "/Game/Afterlife/Core/BattleSystem/BPI_Damagable.BPI_Damagable_C")
                  (message `/Game/Afterlife/Core/BattleSystem/BPI_Damagable.TakeDamage` _hitactor (`self.WeaponDamage`) (`self.DamageType`) (`self.PushDistance`) _userref (`self.K2_GetActorLocation` _userref))))
              (`KismetSystemLibrary.Delay` _tempfirerate)
              (goto _label :!via `Reset`)))
          (else
            (`KismetSystemLibrary.PrintString` "No ammo")
            (`KismetSystemLibrary.Delay` _tempfirerate)
            (goto _label :!via `Reset`)))))))

(event `UpdateAmmoCount`
  (set `self.InventotyAmmo` 0)
  (for _array_element (`InventoryComponent.InventorySlots` (`MainCharacter.GetInventoryComponent` (`self.UserRef`)))
    (bind (_item _quantity) (break `InventorySlot` _array_element))
    (if (== (break `Item` _item) (`self.AmmoType`))
      (set `self.InventotyAmmo` (+ (`self.InventotyAmmo`) _quantity)))))

(event `self.StartAltAction`)

(event `self.Reload`
  (params (AmmoCount :type Integer))
  (`self.UpdateAmmoCount`)
  (set `self.CanShoot` false)
  (`self.StartReloadAnim`)
  (set `self.InventotyAmmo` (`KismetMathLibrary.Max` (- (`self.InventotyAmmo`) (- (`self.MaxAmmo`) (`self.CurrentAmmo`)))))
  (for (_array_element _array_index) (`InventoryComponent.InventorySlots` (`MainCharacter.GetInventoryComponent` (`self.UserRef`)))
    (bind (_item _quantity) (break `InventorySlot` _array_element))
    (if (== (break `Item` _item) (`self.AmmoType`))
      (if (>= _quantity (- (`self.MaxAmmo`) (`self.CurrentAmmo`)))
        (bind (_item_2 _quantity_2) (break `InventorySlot` _array_element))
        (`KismetArrayLibrary.Array_Set` (`InventoryComponent.InventorySlots` (`MainCharacter.GetInventoryComponent` (`self.UserRef`))) _array_index (make `InventorySlot` _item_2 (- _quantity_2 (- (`self.MaxAmmo`) (`self.CurrentAmmo`)))))
        (set `self.CurrentAmmo` (`self.MaxAmmo`))
        (break)
        (else
          (set `self.CurrentAmmo` (+ (`self.CurrentAmmo`) _quantity))
          (`KismetArrayLibrary.Array_Set` (`InventoryComponent.InventorySlots` (`MainCharacter.GetInventoryComponent` (`self.UserRef`))) _array_index (make `InventorySlot` (struct :`DisplayName` "NOT DEFINED" :`MaxStackSize` 1)))))))
  (`KismetSystemLibrary.Delay` (`self.ReloadTime`))
  (set `self.CanShoot` true)
  (`/Game/Afterlife/Framework/Player/BP_MainCharacter.ChangeAmmoCount` (`self.UserRef`) (`self.CurrentAmmo`) (`self.InventotyAmmo`)))

(event `StartReloadAnim`
  ; Определяется в наследниках
)

(event `FireAnim`
  ; определяется в наследниках
  (`|PlayMontage` (`Character.Mesh` (`self.UserRef`)) "/Game/Afterlife/Art/Characters/Player_Character/AM_Shoot.AM_Shoot"
    (:`then`
      (`AISense_Hearing.ReportNoiseEvent` (`self.K2_GetActorLocation`) 100.0 (`self.UserRef`) 100.0))))

(event `HiEffect`
  (params (Location :type "Vector Structure"))
  (bind _fireeffectemmiter (`self.FireEffectEmmiter`))
  ; Эффект попадания
  (bind _returnvalue (`NiagaraFunctionLibrary.SpawnSystemAtLocation` (`self.ShotEffect`) (`SceneComponent.K2_GetComponentLocation` _fireeffectemmiter) (`SceneComponent.K2_GetComponentRotation` _fireeffectemmiter) (1.0 1.0 1.0) false true "None" false)) ; Вспышка перед оружием
  (`PlayerController.ClientStartCameraShake` :`self` (`GameplayStatics.GetPlayerController` 0) :`Shake` (`self.Camera_Shaker`))
  (set `SceneComponent.bAbsoluteLocation` false _returnvalue)
  (`SceneComponent.K2_AttachToComponent` _returnvalue (`self.FireEffectEmmiter`) "None" "SnapToTarget" "KeepRelative" "SnapToTarget" false)
  (`GameplayStatics.SpawnEmitterAtLocation` (`self.HitEffect`) Location (struct) (0.4 0.4 0.4)) ; По поверхности
  (`GameplayStatics.PlaySoundAtLocation` "/Game/Afterlife/Sounds/Impacts/SW_Hit_Impact_1_Cue.SW_Hit_Impact_1_Cue" Location (struct) 1.0 1.0 0.0 null null null null))

(fn `CheckPlayerAmmo`
  (params (UserRef :type "/Game/Afterlife/Framework/Player/BP_MainCharacter Object Reference"))
  (returns (AmmoID :type Name))
  (return "None"))

(fn `PerformBurstShot`
  (if (> (`self.CurrentAmmo`) 0)
    (`IMainAction.StartMainAction`)
    (else
      (`self.StopBurst`))))

(fn `StartBursting`
  (if (> (`self.CurrentAmmo`) 0)
    (set `self.IsBursting` true)
    (`IMainAction.StartMainAction`)
    (bind _returnvalue (`KismetSystemLibrary.K2_SetTimer` null "PerformBurstShot" (`self.FireRateBurst`) true))
    (set `self.BurstTimerHandler` _returnvalue)))

(fn `StopBurst`
  (`KismetSystemLibrary.K2_ClearAndInvalidateTimerHandle` (`self.BurstTimerHandler`))
  (set `self.IsBursting` false))

(fn `UserConstructionScript`
  (`parent.UserConstructionScript`))
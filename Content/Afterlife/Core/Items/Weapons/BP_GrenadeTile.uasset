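; BP_GrenadeTile is a thrown grenade actor, configured through Init with mesh, damage, radius, pushing force and thrower, and propelled by an impulse in Launch.
; Its first hit freezes physics and starts Boom!, which plays a charge-up effect, then a delayed explosion with sound.
; After a hard-coded delay (GrenadeDelay is only stored), a sphere overlap sends damage and push to BPI_Damagable actors, then the grenade destroys itself.
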(event `self.ReceiveBeginPlay`
  (`PrimitiveComponent.SetSimulatePhysics` (`self.StaticMesh`) true))

(event `Boom!`
  (`self.VFXEvent`)
  (`KismetSystemLibrary.Delay` 2.0)
  (bind _outactors (`KismetSystemLibrary.SphereOverlapActors` (`SceneComponent.K2_GetComponentLocation` (`self.StaticMesh`)) (`self.Radius`) (`|MakeArray`) "/Script/Engine.Actor"))
  (for _array_element _outactors
    (if (`KismetSystemLibrary.DoesImplementInterface` _array_element "/Game/Afterlife/Core/BattleSystem/BPI_Damagable.BPI_Damagable_C")
      (message `/Game/Afterlife/Core/BattleSystem/BPI_Damagable.TakeDamage` _array_element (`self.Damage`) "NewEnumerator0" (`self.PushingForce`) (`self.UserRef`) (stale `VFXEvent` _output_get))
      (`KismetSystemLibrary.PrintString` "Hello")))
  (`self.K2_DestroyActor`))

(event `Launch`
  (params (Impulse :type "Vector Structure"))
  (`PrimitiveComponent.AddImpulse` (`self.StaticMesh`) Impulse "None" false))

(event `VFXEvent`
  (bind _returnvalue (`SceneComponent.K2_GetComponentLocation` (`self.StaticMesh`)))
  (`NiagaraFunctionLibrary.SpawnSystemAtLocation` "/Game/Afterlife/VFX/Packs/Mixed_Magic_VFX_Pack/VFX/NS_Magma_Shot_Owner_Cast_Spell.NS_Magma_Shot_Owner_Cast_Spell" _returnvalue (struct) (10000.0 10000.0 10000.0))
  (bind _output_get (set `self.TempLocation` _returnvalue))
  (`GameplayStatics.PlaySoundAtLocation` "/Game/Afterlife/Sounds/Guns/Grenade/Grenade_PowerUp_Cue.Grenade_PowerUp_Cue" _output_get (struct) 1.0 1.0 0.0 null null null null)
  (`KismetSystemLibrary.Delay` 1.5)
  (`NiagaraFunctionLibrary.SpawnSystemAtLocation` "/Game/Afterlife/VFX/Packs/Mixed_Magic_VFX_Pack/VFX/NS_Magma_Shot.NS_Magma_Shot" _output_get (struct) (4.0 4.0 4.0))
  (`GameplayStatics.PlaySoundAtLocation` "/Game/Afterlife/Sounds/Guns/Grenade/CUE/Weapon_Grenade_Explosion_Cue.Weapon_Grenade_Explosion_Cue" _output_get (struct) 2.0 1.0 0.0 null null null null))

(event `self.StaticMesh.OnComponentHit`
  (params (HitComponent :type "PrimitiveComponent Object Reference") (OtherActor :type "Actor Object Reference") (OtherComp :type "PrimitiveComponent Object Reference") (NormalImpulse :type "Vector Structure") (Hit :type "HitResult Structure (by ref)"))
  (`/Engine/EditorBlueprintResources/StandardMacros.DoOnce` false
    (:`Completed`
      (`KismetSystemLibrary.PrintString` "Hit")
      (`self.Boom!`)
      (`PrimitiveComponent.SetSimulatePhysics` (`self.StaticMesh`) false))))

(fn `Init`
  (params (Damage :type "Float (double-precision)") (Mesh :type "StaticMesh Object Reference") (Radius :type "Float (double-precision)") (GrenadeDelay :type "Float (double-precision)") (PushingForce :type "Float (double-precision)") (Thrower :type "Pawn Object Reference"))
  (set `self.PushingForce` PushingForce)
  (set `self.Damage` Damage)
  (set `self.Radius` Radius)
  (`StaticMeshComponent.SetStaticMesh` (`self.StaticMesh`) Mesh)
  (`PrimitiveComponent.SetSimulatePhysics` (`self.StaticMesh`) true)
  (set `self.GrenadeDelay` GrenadeDelay)
  (set `self.UserRef` Thrower))

(fn `NewFunction`)

(fn `UserConstructionScript`)
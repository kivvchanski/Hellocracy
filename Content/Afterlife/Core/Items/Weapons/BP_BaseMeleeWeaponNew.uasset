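; Base melee weapon actor that performs a player attack with montage, Niagara effect, sounds and camera shake, then destroys itself when the montage completes.
; StartMainAction triggers the swing through a DoOnce, which resets after an attack delay following the damage check.
; The montage's "Damage" notify sends TakeDamageMessage with push distance to BPI_Damagable actors overlapping DamageCollision, excluding the user, and plays a hit or miss sound.
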(event `DamageEvent`
  (bind _userref (`self.UserRef`))
  (set `self.bHit` false)
  (for _array_element (`PrimitiveComponent.GetOverlappingActors` (`self.DamageCollision`) "/Script/Engine.Actor")
    (if (`KismetSystemLibrary.DoesImplementInterface` _array_element "/Game/Afterlife/Core/BattleSystem/BPI_Damagable.BPI_Damagable_C")
      (if (!= _array_element (`self.UserRef`))
        (set `self.bHit` true)
        (message `/Game/Afterlife/Core/BattleSystem/BPI_Damagable.TakeDamage` _array_element (`self.WeaponDamage`) (`self.DamageType`) (`self.PushDistance`) _userref (`self.K2_GetActorLocation` _userref))
        (`KismetSystemLibrary.PrintString` "TakeDamage"))))
  (if (`self.bHit`)
    (set `self.HitSound` "/Game/Afterlife/Sounds/Guns/Suitcase/Melee_Full_Punch_NEW.Melee_Full_Punch_NEW")
    (else
      (set `self.HitSound` "/Game/Afterlife/Sounds/Guns/Suitcase/Melee_Miss_NEW.Melee_Miss_NEW")))
  (`GameplayStatics.PlaySound2D` (`self.HitSound`) 1.0 1.0 0.0 null null)
  (`KismetSystemLibrary.Delay` (`self.AtackDelay`))
  (goto _label :!via `Reset`))

(event `self.StartMainAction`
  (`/Engine/EditorBlueprintResources/StandardMacros.DoOnce` false :!label _label
    (:`Completed`
      (`self.PlayAtackAnim`))))

(event `self.OnEquip`)

(event `PlayAtackAnim`
  (bind _damagecollision (`self.DamageCollision`))
  (`NiagaraFunctionLibrary.SpawnSystemAtLocation` null (`SceneComponent.K2_GetComponentLocation` _damagecollision) (`SceneComponent.K2_GetComponentRotation` _damagecollision) (0.3 0.3 0.3)) ; Удар ближний бой
  (`GameplayStatics.PlaySound2D` "/Game/Afterlife/Sounds/Impacts/Player/Player_Attack_Close.Player_Attack_Close" 1.0 1.0 0.0 null null)
  (`GameplayStatics.PlaySound2D` "/Game/Afterlife/Sounds/Guns/Suitcase/Melee_Wing.Melee_Wing" 1.0 1.0 0.0 null null)
  (`PlayerController.ClientStartCameraShake` :`self` (`GameplayStatics.GetPlayerController` 0) :`Shake` (`self.Camera_Shaker_Melee`) :`PlaySpace` "World")
  (bind _notifyname (`|PlayMontage` (`Character.Mesh` (`self.UserRef`)) "/Game/Afterlife/Art/Characters/Player_Character/AS_Player_Char02_Toothy_Hit1_Montage.AS_Player_Char02_Toothy_Hit1_Montage" 0.8)
    (:`OnCompleted`
      (`self.K2_DetachFromActor` "KeepWorld" "KeepWorld" "KeepWorld")
      (`self.K2_DestroyActor`))
    (:`OnNotifyBegin`
      (if (== _notifyname "Damage")
        (`self.DamageEvent`)))))

(fn `UserConstructionScript`
  (`parent.UserConstructionScript`))
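; Base melee weapon Blueprint that plays a montage attack and damages actors inside its collision.
; On equip it attaches the damage collision to the user's view point and triggers a weapon change.
; The main action, gated by a DoOnce, plays effects, camera shake and the montage.
; A "Damage" notify plays hit sounds and damages overlapping damageable actors except the user, then reopens the gate after an attack delay.
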(event `DamageEvent`
  (bind _userref (`self.UserRef`))
  (for _array_element (`PrimitiveComponent.GetOverlappingActors` (`self.DamageCollision`) "/Script/Engine.Actor")
    (if (`KismetSystemLibrary.DoesImplementInterface` _array_element "/Game/Afterlife/Core/BattleSystem/BPI_Damagable.BPI_Damagable_C")
      (if (!= _array_element (`self.UserRef`))
        (message `/Game/Afterlife/Core/BattleSystem/BPI_Damagable.TakeDamage` _array_element (`self.WeaponDamage`) (`self.DamageType`) (`self.PushDistance`) _userref (`self.K2_GetActorLocation` _userref))
        (`KismetSystemLibrary.PrintString` "TakeDamage"))))
  (`KismetSystemLibrary.Delay` (`self.AtackDelay`))
  (goto _label :!via `Reset`))

(event `self.StartMainAction`
  (`/Engine/EditorBlueprintResources/StandardMacros.DoOnce` false :!label _label
    (:`Completed`
      (`self.PlayAtackAnim`))))

(event `self.OnEquip`
  (bind _userref (`self.UserRef`))
  (`SceneComponent.K2_AttachToComponent` (`self.DamageCollision`) (`/Game/Afterlife/Framework/Player/BP_MainCharacter.ViewPoint` _userref) "None" "KeepRelative" "KeepRelative" "KeepRelative" true)
  (`/Game/Afterlife/Framework/Player/BP_MainCharacter.ChangeWeapon` _userref true))

(event `PlayAtackAnim`
  (bind _damagecollision (`self.DamageCollision`))
  (`NiagaraFunctionLibrary.SpawnSystemAtLocation` null (`SceneComponent.K2_GetComponentLocation` _damagecollision) (`SceneComponent.K2_GetComponentRotation` _damagecollision) (0.3 0.3 0.3)) ; Удар ближний бой
  (`PlayerController.ClientStartCameraShake` :`self` (`GameplayStatics.GetPlayerController` 0) :`Shake` (`self.Camera_Shaker_Melee`) :`PlaySpace` "World")
  (bind _notifyname (`|PlayMontage` (`Character.Mesh` (`self.UserRef`)) "/Game/Afterlife/Art/Characters/Player_Character/AM_MeleeAtack.AM_MeleeAtack")
    (:`OnNotifyBegin`
      (if (== _notifyname "Damage")
        (`self.DamageEvent`)
        (`GameplayStatics.PlaySound2D` "/Game/Afterlife/Sounds/Impacts/Player/Player_Attack_Close.Player_Attack_Close" 1.0 1.0 0.0 null null)
        (`GameplayStatics.PlaySound2D` "/Game/Afterlife/Sounds/Guns/Suitcase/Suitcase_Hit_1.Suitcase_Hit_1" 1.0 1.0 0.0 null null)))))

(fn `UserConstructionScript`
  (`parent.UserConstructionScript`))
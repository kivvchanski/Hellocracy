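; A pickable potion bottle item that restores health to the main character when interacted with.
; On Interact it runs the parent logic, casts the interacting actor to BP_MainCharacter, and adds Heal to CurrentHP, clamped to MaxHP.
; The construction script only calls the parent, and the BeginPlay, overlap and Tick events are disabled stubs.
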(event `/Game/Afterlife/Core/InteractionSystem/BP_BaseInteractionObject.Interact`
  (params (InteractingActor :type "MainCharacter Object Reference"))
  (`parent.Interact` InteractingActor)
  (bind _asbp_main_character (cast `/Game/Afterlife/Framework/Player/BP_MainCharacter` InteractingActor))
  (set `/Game/Afterlife/Framework/Player/BP_MainCharacter.CurrentHP` (`KismetMathLibrary.FMin` (`/Game/Afterlife/Framework/Player/BP_MainCharacter.MaxHP` _asbp_main_character) (+ (`/Game/Afterlife/Framework/Player/BP_MainCharacter.CurrentHP` _asbp_main_character) (`self.Heal`))) _asbp_main_character))

(fn `UserConstructionScript`
  (`parent.UserConstructionScript`))
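; Base pickable item actor that players focus to see a name and quantity prompt, then interact with to collect.
; Loads item info from a data table row, optionally attaches to another item's mesh, and registers with the GameState spawner when respawn is enabled.
; Soul-bound items go to GameInstance quest items, others to the interactor's inventory component.
; The inventory path destroys the actor even when adding fails.
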(event `self.ReceiveBeginPlay`
  (bind _itemtoattach (`self.ItemToAttach`))
  (bind (_datatable _rowname) (break `DataTableRowHandle` (`self.TableRowRef`)))
  (`KismetSystemLibrary.DelayUntilNextTick`)
  (if (`self.Respawn`)
    (`self.Init`))
  (`parent.ReceiveBeginPlay`)
  (`/Engine/EditorBlueprintResources/StandardMacros.IsValid` _itemtoattach
    (:`Is Valid`
      (`self.K2_AttachToComponent` (`/Game/Afterlife/Core/InteractionSystem/BP_BaseInteractionObject.StaticMesh` _itemtoattach) "None" "KeepRelative" "KeepRelative" "KeepRelative"))
    (:`Is Not Valid`
      _))
  (`/Engine/EditorBlueprintResources/StandardMacros.IsValid` _datatable
    (:`Is Valid`
      (bind _returnvalue (`|GetDataTableRow` _datatable _rowname)
        (:`then`
          (set `self.ItemInfo` _returnvalue))))
    (:`Is Not Valid`
      (`KismetSystemLibrary.PrintString` (`KismetSystemLibrary.GetObjectName` self)))))

(event `InteractableInterface.Interact`
  (params (InteractingActor :type "MainCharacter Object Reference"))
  (bind _returnvalue (`MainCharacter.GetInventoryComponent` InteractingActor))
  (bind _iteminfo_itemid (break `Item` (`self.ItemInfo`)))
  (bind (_itemid _displayname _bissoulbound) (break `Item` (`self.ItemInfo`)))
  (if _bissoulbound
    (bind _asbp_game_instance (cast `/Game/Afterlife/Framework/BP_GameInstance` (`GameplayStatics.GetGameInstance`)))
    (`/Game/Afterlife/Framework/BP_GameInstance.AddQuestItem` _asbp_game_instance _itemid)
    (else
      (`/Engine/EditorBlueprintResources/StandardMacros.IsValid` _returnvalue
        (:`Is Valid`
          (bind _returnvalue_2 (`InventoryComponent.AddItem` _returnvalue (`self.ItemInfo`) (`self.Quantity`)))
          (if _returnvalue_2
            (`KismetSystemLibrary.PrintString` (`KismetStringLibrary.Concat_StrStr` "PickUpItem" (`KismetTextLibrary.Conv_TextToString` (`KismetTextLibrary.Conv_NameToText` _iteminfo_itemid))))
            (else
              (`KismetSystemLibrary.PrintString` "InventoryFull")))
          (`parent.Interact` null)
          (bind _asbp_main_character (cast `/Game/Afterlife/Framework/Player/BP_MainCharacter` InteractingActor))
          (`/Game/Afterlife/Framework/Player/BP_MainCharacter.OnPickUpUpdate` _asbp_main_character)))))
  (`self.K2_DestroyActor`)
  (`InteractableInterface.OnFocusEnd` InteractingActor))

(event `InteractableInterface.OnFocusStart`
  (params (InteractingActor :type "MainCharacter Object Reference"))
  (bind (_iteminfo_itemid _iteminfo_displayname) (break `Item` (`self.ItemInfo`)))
  (bind _asbp_main_character (cast `/Game/Afterlife/Framework/Player/BP_MainCharacter` InteractingActor))
  (`/Game/Afterlife/Framework/Player/BP_MainCharacter.AddInteractionText` _asbp_main_character (`KismetStringLibrary.Concat_StrStr` "Взять: " (`KismetStringLibrary.Conv_IntToString` (`self.Quantity`)) " " (`KismetTextLibrary.Conv_TextToString` _iteminfo_displayname))))

(event `InteractableInterface.OnFocusEnd`
  (params (InteractingActor :type "MainCharacter Object Reference"))
  (bind _asbp_main_character (cast `/Game/Afterlife/Framework/Player/BP_MainCharacter` InteractingActor))
  (`/Game/Afterlife/Framework/Player/BP_MainCharacter.HideInteractionText` _asbp_main_character))

(fn `Init`
  (bind _asbp_game_state (cast `/Game/Afterlife/Framework/BP_GameState` (`GameplayStatics.GetGameState`)))
  (`/Game/Afterlife/Core/BattleSystem/Enemies/Utils/BP_Spawner.AddItemSpawner` (`/Game/Afterlife/Framework/BP_GameState.Spawner` _asbp_game_state) (`self.GetTransform`) (make `/Game/Afterlife/Core/BattleSystem/Enemies/Utils/F_LandingItems` (`GameplayStatics.GetObjectClass` self) (`self.ItemToAttach`) (`self.Quantity`)) self))

(fn `UserConstructionScript`
  (`parent.UserConstructionScript`))
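; BP_Trap is a trigger trap that temporarily roots the main character on contact with its box.
; While armed, overlap disarms it, blocks dashing and disables movement, then restores walking and dash after EffectDuration.
; The character leaving the box starts CooldownDuration, after which the trap re-arms.
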(event `self.Box.OnComponentBeginOverlap`
  (params (OverlappedComponent :type "PrimitiveComponent Object Reference") (OtherActor :type "Actor Object Reference") (OtherComp :type "PrimitiveComponent Object Reference") (OtherBodyIndex :type Integer) (bFromSweep :type Boolean) (SweepResult :type "HitResult Structure (by ref)"))
  (bind _asbp_main_character (cast `/Game/Afterlife/Framework/Player/BP_MainCharacter` OtherActor))
  (if (`self.bTrapActive`)
    (set `/Game/Afterlife/Framework/Player/BP_MainCharacter.bCanDash` false _asbp_main_character)
    (set `self.bTrapActive` false)
    (set `self.bPlayerInside` true)
    (bind _output_get (set `self.TrappedCharacter` _asbp_main_character))
    (bind _movecomp (`/Game/Afterlife/Framework/Player/BP_MainCharacter.GetCharacterMovement` _output_get))
    (`CharacterMovementComponent.DisableMovement` _movecomp)
    (`KismetSystemLibrary.Delay` (`self.EffectDuration`))
    (`CharacterMovementComponent.SetMovementMode` _movecomp "MOVE_Walking" 0)
    (set `/Game/Afterlife/Framework/Player/BP_MainCharacter.bCanDash` true _output_get)))

(event `self.Box.OnComponentEndOverlap`
  (params (OverlappedComponent :type "PrimitiveComponent Object Reference") (OtherActor :type "Actor Object Reference") (OtherComp :type "PrimitiveComponent Object Reference") (OtherBodyIndex :type Integer))
  (cast `/Game/Afterlife/Framework/Player/BP_MainCharacter` OtherActor)
  (set `self.bPlayerInside` false)
  (`KismetSystemLibrary.Delay` (`self.CooldownDuration`))
  (set `self.bTrapActive` true))

(fn `UserConstructionScript`)
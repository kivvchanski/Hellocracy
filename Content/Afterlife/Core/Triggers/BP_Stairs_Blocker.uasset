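; BP_Stairs_Blocker is a blocker, by its name for stairs, that moves vertically when a monitored enemy dies.
; On BeginPlay it binds to EnemyToMonitor's death event, which plays a timeline from the start.
; Each timeline update adds the Walls track value to the Scene component's current relative Z, so the offset accumulates per update, teleporting without sweep.
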(event `self.ReceiveBeginPlay`
  (add `/Game/Afterlife/Core/BattleSystem/Enemies/BP_BaseEnemy.OnEnemyDied` (`self.EnemyToMonitor`) (delegate `CustomEvent`)))

(event `CustomEvent`
  (bind (_direction _walls) (`Timeline|Timeline` :!via `PlayFromStart`)
    (:`Update`
      (`SceneComponent.K2_SetRelativeLocation` (`self.Scene`) (`KismetMathLibrary.MakeVector` (.x (`SceneComponent.RelativeLocation` (`self.Scene`))) (.y (`SceneComponent.RelativeLocation` (`self.Scene`))) (+ _walls (.z (`SceneComponent.RelativeLocation` (`self.Scene`))))) false true))))

(fn `UserConstructionScript`)
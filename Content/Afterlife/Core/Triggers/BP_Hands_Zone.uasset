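; BP_Hands_Zone is a trigger zone of grabbing hands that slows the main character while inside.
; On box overlap it applies custom time dilation, allows dashing, flags the hands' anim Blueprint, shows the WBP_In_Hands widget and switches the looping idle sound to a walk cue.
; Leaving restores speed, sound and animation flag and removes the widget.
; GetDash exposes the trapped character's dash state; a timed movement-disable chain is left unconnected.
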(event `self.ReceiveBeginPlay`
  (`AudioComponent.Play` (`self.Hands_Idle_Cue`) 0.0))

(event `self.Box.OnComponentBeginOverlap`
  (params (OverlappedComponent :type "PrimitiveComponent Object Reference") (OtherActor :type "Actor Object Reference") (OtherComp :type "PrimitiveComponent Object Reference") (OtherBodyIndex :type Integer) (bFromSweep :type Boolean) (SweepResult :type "HitResult Structure (by ref)"))
  (bind _asbp_main_character (cast `/Game/Afterlife/Framework/Player/BP_MainCharacter` OtherActor))
  (`AudioComponent.SetSound` (`self.Hands_Idle_Cue`) "/Game/Afterlife/Sounds/Impacts/Hands_Walk_Cue.Hands_Walk_Cue")
  (bind _asabp_catch_hands (cast `/Game/Afterlife/Art/Characters/Catch_hands/ABP_Catch_Hands` (`SkeletalMeshComponent.GetAnimInstance` (`self.SkeletalMesh`))))
  (set `/Game/Afterlife/Art/Characters/Catch_hands/ABP_Catch_Hands.bPlayerInside` true _asabp_catch_hands)
  (bind _returnvalue (`|CreateWidget` "/Game/Afterlife/UI/Widget_Zone_Icons/WBP_In_Hands.WBP_In_Hands_C"))
  (`UserWidget.AddToViewport` _returnvalue 0)
  (set `Actor.CustomTimeDilation` 0.35 _asbp_main_character)
  (set `self.bPlayerInside` true)
  (bind _output_get (set `self.TrappedCharacter` _asbp_main_character))
  (set `/Game/Afterlife/Framework/Player/BP_MainCharacter.bCanDash` true _output_get))

(event `self.Box.OnComponentEndOverlap`
  (params (OverlappedComponent :type "PrimitiveComponent Object Reference") (OtherActor :type "Actor Object Reference") (OtherComp :type "PrimitiveComponent Object Reference") (OtherBodyIndex :type Integer))
  (bind _asbp_main_character (cast `/Game/Afterlife/Framework/Player/BP_MainCharacter` OtherActor))
  (`AudioComponent.SetSound` (`self.Hands_Idle_Cue`) "/Game/Afterlife/Sounds/Impacts/Hands_Idle_New_Cue.Hands_Idle_New_Cue")
  (set `/Game/Afterlife/Art/Characters/Catch_hands/ABP_Catch_Hands.bPlayerInside` false (stale `self.Box.OnComponentBeginOverlap` _asabp_catch_hands))
  (`Widget.RemoveFromParent` (stale `self.Box.OnComponentBeginOverlap` _returnvalue))
  (set `self.bPlayerInside` false)
  (set `Actor.CustomTimeDilation` 1.0 _asbp_main_character))

(fn `getDash`
  (returns (`can dash` :type Boolean))
  (bind _asbp_main_character (cast `/Game/Afterlife/Framework/Player/BP_MainCharacter` (`self.TrappedCharacter`)))
  (return (`/Game/Afterlife/Framework/Player/BP_MainCharacter.bCanDash` _asbp_main_character)))

(fn `UserConstructionScript`)
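; BP_DamageZoneBIG is a trigger volume that periodically damages BP_MainCharacter while it is inside.
; Box overlap, plus a short-delayed BeginPlay check for characters already inside, plays an entry sound, shows the WBP_In_DamageZone widget and starts a looping DealDamage timer.
; The widget reference guards against duplicate timers; leaving clears the timer, plays an exit sound and removes the widget.
; A RegenHealth event exists but is never called here.
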(event `self.ReceiveBeginPlay`
  (`KismetSystemLibrary.Delay` 0.2)
  (for _array_element (`self.GetOverlappingActors` "/Game/Afterlife/Framework/Player/BP_MainCharacter.BP_MainCharacter_C")
    (set `self.PlayerRef` _array_element)
    (`/Engine/EditorBlueprintResources/StandardMacros.IsValid` (`self.WBP_Icon`)
      (:`Is Not Valid`
        (`GameplayStatics.PlaySound2D` "/Game/Afterlife/Framework/Damage_zone/damagezonein.damagezonein" 1.0 1.0 0.0 null null)
        (bind _returnvalue (`|CreateWidget` "/Game/Afterlife/UI/Widget_Zone_Icons/WBP_In_DamageZone.WBP_In_DamageZone_C"))
        (bind _output_get (set `self.WBP_Icon` _returnvalue))
        (`UserWidget.AddToViewport` _output_get 0)
        (bind _returnvalue_2 (`KismetSystemLibrary.K2_SetTimerDelegate` (delegate `DealDamage`) (`self.TickInterval`) true))
        (set `self.DamageTimerHandle` _returnvalue_2)))))

(event `DealDamage`
  (`/Game/Afterlife/Framework/Player/BP_MainCharacter.TakeDamageinZone` (`self.PlayerRef`) (`self.DamagePerTick`) "NewEnumerator0" 0.0 null (0.0 0.0 0.0)))

(event `self.Box Collision.OnComponentBeginOverlap`
  (params (OverlappedComponent :type "PrimitiveComponent Object Reference") (OtherActor :type "Actor Object Reference") (OtherComp :type "PrimitiveComponent Object Reference") (OtherBodyIndex :type Integer) (bFromSweep :type Boolean) (SweepResult :type "HitResult Structure (by ref)"))
  (bind _asbp_main_character (cast `/Game/Afterlife/Framework/Player/BP_MainCharacter` OtherActor))
  (set `self.PlayerRef` _asbp_main_character)
  (`/Engine/EditorBlueprintResources/StandardMacros.IsValid` (`self.WBP_Icon`)
    (:`Is Not Valid`
      (`GameplayStatics.PlaySound2D` "/Game/Afterlife/Framework/Damage_zone/damagezonein.damagezonein" 1.0 1.0 0.0 null null)
      (bind _returnvalue (`|CreateWidget` "/Game/Afterlife/UI/Widget_Zone_Icons/WBP_In_DamageZone.WBP_In_DamageZone_C"))
      (bind _output_get (set `self.WBP_Icon` _returnvalue))
      (`UserWidget.AddToViewport` _output_get 0)
      (bind _returnvalue_2 (`KismetSystemLibrary.K2_SetTimerDelegate` (delegate `DealDamage`) (`self.TickInterval`) true))
      (set `self.DamageTimerHandle` _returnvalue_2))))

(event `RegenHealth`
  (bind _playerref (`self.PlayerRef`))
  (set `/Game/Afterlife/Framework/Player/BP_MainCharacter.CurrentHP` (+ (`/Game/Afterlife/Framework/Player/BP_MainCharacter.CurrentHP` _playerref) (`self.RegenPerTick`)) _playerref))

(event `self.Box Collision.OnComponentEndOverlap`
  (params (OverlappedComponent :type "PrimitiveComponent Object Reference") (OtherActor :type "Actor Object Reference") (OtherComp :type "PrimitiveComponent Object Reference") (OtherBodyIndex :type Integer))
  (bind _asbp_main_character (cast `/Game/Afterlife/Framework/Player/BP_MainCharacter` OtherActor))
  (set `self.PlayerRef` _asbp_main_character)
  (`KismetSystemLibrary.K2_ClearAndInvalidateTimerHandle` (`self.DamageTimerHandle`))
  (`/Engine/EditorBlueprintResources/StandardMacros.IsValid` (`self.WBP_Icon`)
    (:`Is Valid`
      (`GameplayStatics.PlaySound2D` "/Game/Afterlife/Framework/Damage_zone/damagezoneout.damagezoneout" 1.0 1.0 0.0 null null)
      (`Widget.RemoveFromParent` (`self.WBP_Icon`))
      (set `self.WBP_Icon` null))))

(fn `UserConstructionScript`)
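; BP_Trigger_Boss_Pit is a trigger that starts a boss encounter the first time the player pawn enters it.
; Entry swaps the Door for a QuestDoor, plays a sound and shows a boss health bar.
; The bar follows EnemyToMonitor's health through bound events.
; On the enemy's death it removes the bar, respawns the original door class at the saved transform and drives sound volume by timeline before stopping it.
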(event `self.Trigger_0.OnComponentBeginOverlap`
  (params (OverlappedComponent :type "PrimitiveComponent Object Reference") (OtherActor :type "Actor Object Reference") (OtherComp :type "PrimitiveComponent Object Reference") (OtherBodyIndex :type Integer) (bFromSweep :type Boolean) (SweepResult :type "HitResult Structure (by ref)"))
  (bind _door (`self.Door`))
  (bind _enemytomonitor (`self.EnemyToMonitor`))
  (if (== OtherActor (`GameplayStatics.GetPlayerPawn` 0))
    (`/Engine/EditorBlueprintResources/StandardMacros.DoOnce` false
      (:`Completed`
        (bind _output_get (set `self.DoorTransform` (`self.GetTransform` _door)))
        (`self.K2_DestroyActor` _door)
        (bind _returnvalue (`|SpawnActorFromClass` (`self.QuestDoor`) _output_get "Undefined" "MultiplyWithRoot" null null))
        (`KismetSystemLibrary.Delay` 0.2)
        (bind _returnvalue_2 (`GameplayStatics.SpawnSoundAtLocation` (`self.SoundToPlay`) (`self.K2_GetActorLocation`) (struct) 1.0 1.0 0.0 null null))
        (set `self.Sound` _returnvalue_2)
        (bind _returnvalue_3 (`|CreateWidget` "/Game/Afterlife/UI/WBP_BossHealthBar.WBP_BossHealthBar_C"))
        (bind _output_get_2 (set `self.HealthWidget` _returnvalue_3))
        (`/Game/Afterlife/UI/WBP_BossHealthBar.UpdateHealth` _output_get_2 (`/Game/Afterlife/Core/BattleSystem/Enemies/BP_BaseEnemy.CurrentHP` _enemytomonitor) (`/Game/Afterlife/Core/BattleSystem/Enemies/BP_BaseEnemy.MaxHP` _enemytomonitor))
        (`UserWidget.AddToViewport` _output_get_2 0)
        (add `/Game/Afterlife/Core/BattleSystem/Enemies/BP_BaseEnemy.OnHealthChanged` _enemytomonitor (delegate `CustomEvent`))
        (add `/Game/Afterlife/Core/BattleSystem/Enemies/BP_BaseEnemy.OnEnemyDied` (`self.EnemyToMonitor`) (delegate `OnEnemyDiedHandler`))))))

(event `CustomEvent`
  (params (CurrentHP :type "Float (double-precision)") (MaxHP :type "Float (double-precision)"))
  (`/Game/Afterlife/UI/WBP_BossHealthBar.UpdateHealth` (stale `self.Trigger_0.OnComponentBeginOverlap` _output_get_2) CurrentHP MaxHP))

(event `OnEnemyDiedHandler`
  (bind _sound (`self.Sound`))
  (`Widget.RemoveFromParent` (`self.HealthWidget`))
  (set `self.HealthWidget` null)
  (`self.K2_DestroyActor` (stale `self.Trigger_0.OnComponentBeginOverlap` _returnvalue))
  (`|SpawnActorFromClass` (`GameplayStatics.GetObjectClass` (`self.Door`)) (`self.DoorTransform`) "Undefined" "MultiplyWithRoot" null null)
  (bind (_direction _volume) (`Timeline|Timeline_0` :!via `PlayFromStart`)
    (:`Update`
      (`AudioComponent.SetVolumeMultiplier` _sound _volume))
    (:`Finished`
      (`AudioComponent.Stop` _sound))))

(event `self.Trigger_0.OnComponentEndOverlap`
  (params (OverlappedComponent :type "PrimitiveComponent Object Reference") (OtherActor :type "Actor Object Reference") (OtherComp :type "PrimitiveComponent Object Reference") (OtherBodyIndex :type Integer)))

(fn `UserConstructionScript`)
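; BP_FinalPortal is the end-of-level portal, hidden behind walls until activated and completed when the main character enters it.
; ActivatePortal plays opening sound and choir, while a timeline moves the walls vertically by cumulative offsets, then hides them and enables the trigger box.
; When BP_MainCharacter overlaps the box, it prints a placeholder win message, fades the choir and destroys itself after a short delay.
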(event `self.ReceiveBeginPlay`
  (`PrimitiveComponent.SetCollisionEnabled` (`self.Box`) "NoCollision"))

(event `ActivatePortal`
  (bind _walls (`self.Walls`))
  (bind _relativelocation (`SceneComponent.RelativeLocation` (`self.Walls`)))
  (`GameplayStatics.PlaySoundAtLocation` "/Game/Afterlife/Sounds/Environment/WAV/Wall_Opening_Cue.Wall_Opening_Cue" _relativelocation (struct) 1.0 1.0 0.0 null null null null)
  (`AudioComponent.Play` (`self.Choir`) 0.0)
  (bind (_direction _walls_2) (`Timeline|Timeline` :!via `PlayFromStart`)
    (:`Update`
      (`SceneComponent.K2_SetRelativeLocation` (`self.Walls`) (`KismetMathLibrary.MakeVector` (.x _relativelocation) (.y _relativelocation) (+ _walls_2 (.z _relativelocation))) false true))
    (:`Finished`
      (`SceneComponent.SetVisibility` _walls false false)
      (`PrimitiveComponent.SetCollisionEnabled` _walls "NoCollision")
      (`PrimitiveComponent.SetCollisionEnabled` (`self.Box`) "QueryOnly"))))

(event `self.Box.OnComponentBeginOverlap`
  (params (OverlappedComponent :type "PrimitiveComponent Object Reference") (OtherActor :type "Actor Object Reference") (OtherComp :type "PrimitiveComponent Object Reference") (OtherBodyIndex :type Integer) (bFromSweep :type Boolean) (SweepResult :type "HitResult Structure (by ref)"))
  (cast `/Game/Afterlife/Framework/Player/BP_MainCharacter` OtherActor)
  (`KismetSystemLibrary.PrintString` "WINNER WINNER CHICKEN DINNER")
  (`AudioComponent.FadeOut` (`self.Choir`) 2.0 0.0 "Linear")
  (`KismetSystemLibrary.Delay` 0.5)
  (`self.K2_DestroyActor`))

(fn `UserConstructionScript`)
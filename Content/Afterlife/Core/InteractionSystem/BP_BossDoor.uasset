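; BP_BossDoor is an interactable boss door that gates its interaction behind a quest check.
; On Interact, it casts the interacting actor to BP_MainCharacter and passes it to CheckQuest on its BPQuestComponent.
; The parent class's Interact runs only when that check passes, so this child adds just the condition and inherits the interaction behavior itself.
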(event `/Game/Afterlife/Core/InteractionSystem/BP_BaseInteractionObject.Interact`
  (params (InteractingActor :type "MainCharacter Object Reference"))
  (bind _asbp_main_character (cast `/Game/Afterlife/Framework/Player/BP_MainCharacter` InteractingActor))
  (bind _result (`/Game/Afterlife/Core/QuestSystem/BP_QuestComponent.CheckQuest` (`self.BP_QuestComponent`) _asbp_main_character))
  (if _result
    (`parent.Interact` InteractingActor)))

(fn `UserConstructionScript`
  (`parent.UserConstructionScript`))
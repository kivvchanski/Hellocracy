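; BP_Paper is an interactable paper prop that offers the player a read prompt when focused.
; Focus events from the interaction system show the Russian "Читать" (Read) text on BP_MainCharacter and apply the M_Outliner overlay material to the mesh, then clear both when focus ends.
; Interact only prints a debug string and StopInteract is empty, so reading itself is not implemented here.
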(event `self.Interact`
  (params (InteractingActor :type "MainCharacter Object Reference"))
  (`KismetSystemLibrary.PrintString` "Interacted"))

(event `self.OnFocusStart`
  (params (InteractingActor :type "MainCharacter Object Reference"))
  (bind _asbp_main_character (cast `/Game/Afterlife/Framework/Player/BP_MainCharacter` InteractingActor))
  (`/Game/Afterlife/Framework/Player/BP_MainCharacter.AddInteractionText` _asbp_main_character "Читать")
  (`MeshComponent.SetOverlayMaterial` (`self.StaticMesh`) "/Game/Afterlife/Art/Shared/Materials/M_Outliner.M_Outliner"))

(event `self.OnFocusEnd`
  (params (InteractingActor :type "MainCharacter Object Reference"))
  (bind _asbp_main_character (cast `/Game/Afterlife/Framework/Player/BP_MainCharacter` InteractingActor))
  (`/Game/Afterlife/Framework/Player/BP_MainCharacter.HideInteractionText` _asbp_main_character)
  (`MeshComponent.SetOverlayMaterial` (`self.StaticMesh`) null))

(event `self.StopInteract`
  (params (InteractingActor :type "MainCharacter Object Reference")))

(fn `UserConstructionScript`)
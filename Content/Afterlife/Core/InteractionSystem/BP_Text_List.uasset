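; BP_Text_List is an interactable readable text object in the interaction system, responding to BP_MainCharacter.
; Gaining focus shows a "Читать" (Read) prompt on the character and applies M_Outliner as the mesh's overlay material for highlighting.
; Losing focus hides the prompt and clears the overlay.
; Interacting creates a WBP_List widget, passes it TextString and adds it to the viewport.
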(event `self.OnFocusStart`
  (params (InteractingActor :type "MainCharacter Object Reference"))
  (bind _asbp_main_character (cast `/Game/Afterlife/Framework/Player/BP_MainCharacter` InteractingActor))
  (`/Game/Afterlife/Framework/Player/BP_MainCharacter.AddInteractionText` _asbp_main_character "Читать")
  (`MeshComponent.SetOverlayMaterial` (`self.StaticMesh`) "/Game/Afterlife/Art/Shared/Materials/M_Outliner.M_Outliner"))

(event `self.Interact`
  (params (InteractingActor :type "MainCharacter Object Reference"))
  (cast `/Game/Afterlife/Framework/Player/BP_MainCharacter` InteractingActor)
  (bind _returnvalue (`|CreateWidget` "/Game/Afterlife/UI/WBP_List.WBP_List_C"))
  (`/Game/Afterlife/UI/WBP_List.SetString` _returnvalue (`self.Text_String`))
  (`UserWidget.AddToViewport` _returnvalue 0))

(event `InteractableInterface.OnFocusEnd`
  (params (InteractingActor :type "MainCharacter Object Reference"))
  (bind _asbp_main_character (cast `/Game/Afterlife/Framework/Player/BP_MainCharacter` InteractingActor))
  (`MeshComponent.SetOverlayMaterial` (`self.StaticMesh`) "/Game/Afterlife/Art/Shared/Materials/M_Outliner.M_Outliner")
  (`/Game/Afterlife/Framework/Player/BP_MainCharacter.HideInteractionText` _asbp_main_character)
  (`MeshComponent.SetOverlayMaterial` (`self.StaticMesh`) null))

(fn `UserConstructionScript`
  (`parent.UserConstructionScript`))
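; BP_QuestDoor_KitchenOUT is a quest-gated door, apparently the kitchen exit, in the interaction system.
; On Interact by BP_MainCharacter, its quest component's CheckQuest decides whether the door unlocks.
; A passing check plays a card-unlock sound and, after a short delay, calls the parent Interact; a failing check only plays a locked sound.
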(event `/Game/Afterlife/Core/InteractionSystem/BP_BaseInteractionObject.Interact`
  (params (InteractingActor :type "MainCharacter Object Reference"))
  (bind _returnvalue (`self.K2_GetActorLocation`))
  (bind _asbp_main_character (cast `/Game/Afterlife/Framework/Player/BP_MainCharacter` InteractingActor))
  (bind _result (`/Game/Afterlife/Core/QuestSystem/BP_QuestComponent.CheckQuest` (`self.BP_QuestComponent`) _asbp_main_character))
  (if _result
    (`GameplayStatics.PlaySoundAtLocation` "/Game/Afterlife/Sounds/Doors/CUE/Door_Card_Unlock_Cue.Door_Card_Unlock_Cue" _returnvalue (struct) 1.0 1.0 0.0 null null null null)
    (`KismetSystemLibrary.Delay` 0.5)
    (`parent.Interact` InteractingActor)
    (else
      (`GameplayStatics.PlaySoundAtLocation` "/Game/Afterlife/Sounds/Doors/CUE/Door_Locked_Cue.Door_Locked_Cue" _returnvalue (struct) 1.0 1.0 0.0 null null null null))))

(fn `UserConstructionScript`
  (`parent.UserConstructionScript`))
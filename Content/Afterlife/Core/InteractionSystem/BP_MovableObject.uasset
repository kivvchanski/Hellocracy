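; BP_MovableObject is an interactable object, such as something that opens and closes, that toggles between two placements.
; It caches the mesh's world transform at BeginPlay, then Interact plays one of two timelines that lerp it to or from the SecondPosition component's transform.
; The AtStartPosition flag selects the direction and flips on timeline update.
; Focus events show and hide an open/close prompt (in Russian) on BP_MainCharacter.
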(event `self.ReceiveBeginPlay`
  (`parent.ReceiveBeginPlay`)
  (set `self.StartPosition` (`SceneComponent.K2_GetComponentToWorld` (`self.StaticMesh`))))

(event `InteractableInterface.Interact`
  (params (InteractingActor :type "MainCharacter Object Reference"))
  (if (`self.AtStartPosition`)
    (bind (_direction _newtrack_0) (`Timeline|Timeline` :!via `PlayFromStart`)
      (:`Update`
        (`SceneComponent.K2_SetWorldTransform` (`self.StaticMesh`) (`KismetMathLibrary.TLerp` (`self.StartPosition`) (`SceneComponent.K2_GetComponentToWorld` (`self.SecondPosition`)) _newtrack_0) false false)
        (set `self.AtStartPosition` false)))
    (else
      (bind (_direction_2 _newtrack_0_2) (`Timeline|Timeline_0` :!via `PlayFromStart`)
        (:`Update`
          (`SceneComponent.K2_SetWorldTransform` (`self.StaticMesh`) (`KismetMathLibrary.TLerp` (`SceneComponent.K2_GetComponentToWorld` (`self.SecondPosition`)) (`self.StartPosition`) _newtrack_0_2) false false)
          (set `self.AtStartPosition` true))))))

(event `InteractableInterface.OnFocusStart`
  (params (InteractingActor :type "MainCharacter Object Reference"))
  (bind _asbp_main_character (cast `/Game/Afterlife/Framework/Player/BP_MainCharacter` InteractingActor))
  (`/Game/Afterlife/Framework/Player/BP_MainCharacter.AddInteractionText` _asbp_main_character "Открыть/закрыть"))

(event `InteractableInterface.OnFocusEnd`
  (params (InteractingActor :type "MainCharacter Object Reference"))
  (bind _asbp_main_character (cast `/Game/Afterlife/Framework/Player/BP_MainCharacter` InteractingActor))
  (`/Game/Afterlife/Framework/Player/BP_MainCharacter.HideInteractionText` _asbp_main_character))

(fn `UserConstructionScript`
  (`parent.UserConstructionScript`))
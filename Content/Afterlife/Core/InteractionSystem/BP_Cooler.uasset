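; BP_Cooler is a single-use interactable water cooler that heals the player and acts as a checkpoint.
; Focus shows a Russian prompt to drink, or that the water is gone once used.
; The first interaction applies BP_Heal with the character's MaxHP, then, if HP exceeds a threshold, reverses the damage HUD and saves a checkpoint at SpawnPoint.
; It also plays a sip sound, turns off its spotlight and briefly shows a save icon.
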(event `InteractableInterface.OnFocusStart`
  (params (InteractingActor :type "MainCharacter Object Reference"))
  (bind _asbp_main_character (cast `/Game/Afterlife/Framework/Player/BP_MainCharacter` InteractingActor))
  (if (`self.Used`)
    (`/Game/Afterlife/Framework/Player/BP_MainCharacter.AddInteractionText` _asbp_main_character "Вода закончилась")
    (else
      (`/Game/Afterlife/Framework/Player/BP_MainCharacter.AddInteractionText` _asbp_main_character "Попить воды"))))

(event `InteractableInterface.Interact`
  (params (InteractingActor :type "MainCharacter Object Reference"))
  (bind _asbp_main_character (cast `/Game/Afterlife/Framework/Player/BP_MainCharacter` InteractingActor))
  (`/Engine/EditorBlueprintResources/StandardMacros.DoOnce` false
    (:`Completed`
      (set `self.Used` true)
      (bind _returnvalue (`|GenericCreateObject` "/Game/Afterlife/Core/Items/Effects/BP_Heal.BP_Heal_C" (`/Game/Afterlife/Framework/Player/BP_MainCharacter.MaxHP` _asbp_main_character)))
      (`/Game/Afterlife/Core/Items/Effects/BP_BaseEffect.Use` _returnvalue _asbp_main_character)
      (if (> (`/Game/Afterlife/Framework/Player/BP_MainCharacter.CurrentHP` _asbp_main_character) 25.0)
        (set `/Game/Afterlife/Framework/Player/BP_MainCharacter.Should Loop Effect ?` false _asbp_main_character)
        (`/Game/Afterlife/Framework/Player/BP_MainCharacter.Reverse Damage HUD` _asbp_main_character)
        (`/Game/Afterlife/Framework/Player/BP_MainCharacter.SaveCheckpoint` _asbp_main_character (.location (`SceneComponent.K2_GetComponentToWorld` (`self.SpawnPoint`))) (.rotation (`SceneComponent.K2_GetComponentToWorld` (`self.SpawnPoint`)))))
      (`GameplayStatics.PlaySound2D` "/Game/Afterlife/Sounds/Impacts/Player/New_Water_Sip.New_Water_Sip" 1.0 1.0 0.0 null null)
      (`LightComponent.SetIntensity` (`self.SpotLight`) 0.0)
      (bind _returnvalue_2 (`|CreateWidget` "/Game/Afterlife/UI/WBP_SaveIcon.WBP_SaveIcon_C"))
      (`UserWidget.AddToViewport` _returnvalue_2 0)
      (`KismetSystemLibrary.Delay` 2.0)
      (`Widget.RemoveFromParent` _returnvalue_2))))

(fn `UserConstructionScript`
  (`parent.UserConstructionScript`))
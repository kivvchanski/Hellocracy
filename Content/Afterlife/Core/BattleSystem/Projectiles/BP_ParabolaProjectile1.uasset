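; Battle-system projectile that damages the first valid BPI_Damagable actor it overlaps, ignoring its DamageDealer.
; LaunchProjectile sets ProjectileMovement velocity to the unnormalized offset to the target times Speed, so launch speed scales with distance.
; DamageCollision sends damage with type and push distance once, while DestroySphere disables damage on static mesh overlap.
; Both paths fire CallEffect, an empty event here, then destroy the projectile.
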(event `LaunchProjectile`
  (params (TargetPosition :type "Vector Structure"))
  (set `MovementComponent.Velocity` (* (- TargetPosition (`self.K2_GetActorLocation`)) (`self.Speed`)) (`self.ProjectileMovement`)))

(event `self.DamageCollision.OnComponentBeginOverlap`
  (params (OverlappedComponent :type "PrimitiveComponent Object Reference") (OtherActor :type "Actor Object Reference") (OtherComp :type "PrimitiveComponent Object Reference") (OtherBodyIndex :type Integer) (bFromSweep :type Boolean) (SweepResult :type "HitResult Structure (by ref)"))
  (bind _damagedealer (`self.DamageDealer`))
  (if (`self.DealDamage`)
    (`/Engine/EditorBlueprintResources/StandardMacros.IsValid` _damagedealer
      (:`Is Valid`
        (if (!= OtherActor _damagedealer)
          (if (`KismetSystemLibrary.DoesImplementInterface` OtherActor "/Game/Afterlife/Core/BattleSystem/BPI_Damagable.BPI_Damagable_C")
            (`/Engine/EditorBlueprintResources/StandardMacros.DoOnce` false
              (:`Completed`
                (message `/Game/Afterlife/Core/BattleSystem/BPI_Damagable.TakeDamage` OtherActor (`self.Damage`) (`self.DamageType`) (`self.PushingDistance`) (`self.DamageDealer`) (`self.K2_GetActorLocation`))
                (`self.CallEffect`)
                (`self.K2_DestroyActor`))))
          (else
            (`KismetSystemLibrary.PrintString` "Equal")))))))

(event `CallEffect`)

(event `self.DestroySphere.OnComponentBeginOverlap`
  (params (OverlappedComponent :type "PrimitiveComponent Object Reference") (OtherActor :type "Actor Object Reference") (OtherComp :type "PrimitiveComponent Object Reference") (OtherBodyIndex :type Integer) (bFromSweep :type Boolean) (SweepResult :type "HitResult Structure (by ref)"))
  (cast `StaticMeshComponent` OtherComp)
  (set `self.DealDamage` false)
  (`self.CallEffect`)
  (`self.K2_DestroyActor`))

(event `self.DamageCollision.OnComponentHit`
  (params (HitComponent :type "PrimitiveComponent Object Reference") (OtherActor :type "Actor Object Reference") (OtherComp :type "PrimitiveComponent Object Reference") (NormalImpulse :type "Vector Structure") (Hit :type "HitResult Structure (by ref)")))

(event `self.Sphere.OnComponentHit`
  (params (HitComponent :type "PrimitiveComponent Object Reference") (OtherActor :type "Actor Object Reference") (OtherComp :type "PrimitiveComponent Object Reference") (NormalImpulse :type "Vector Structure") (Hit :type "HitResult Structure (by ref)")))

(fn `UserConstructionScript`)
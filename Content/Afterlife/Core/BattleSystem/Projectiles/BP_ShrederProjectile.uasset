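; Shredder projectile for the battle system, whose effect spawns a little enemy that carries a pickup.
; When CallEffect fires, it spawns BP_BaseEnemy_Little at the DamageCollision location.
; A random coin flip sets that enemy's drop to either a bandage or a stack of stapler ammo.
; All other event and construction logic is left to the parent class.
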(event `self.CallEffect`
  (bind _returnvalue (`|SpawnActorFromClass` "/Game/Afterlife/Core/BattleSystem/Enemies/Little/BP_BaseEnemy_Little.BP_BaseEnemy_Little_C" (`KismetMathLibrary.MakeTransform` (`SceneComponent.K2_GetComponentLocation` (`self.DamageCollision`))) "Undefined" "MultiplyWithRoot" null 0.0 10.0 250.0 8.0 1 2.0 false null))
  (if (`KismetMathLibrary.RandomBool`)
    (set `/Game/Afterlife/Core/BattleSystem/Enemies/BP_BaseEnemy.DropItem` "/Game/Afterlife/Core/Items/PickableItems/BP_BasePickableItem_Bandage.BP_BasePickableItem_Bandage_C" _returnvalue)
    (else
      (set `/Game/Afterlife/Core/BattleSystem/Enemies/BP_BaseEnemy.DropItem` "/Game/Afterlife/Core/Items/PickableItems/BP_BasePickableItem_Ammo_Stapler.BP_BasePickableItem_Ammo_Stapler_C" _returnvalue)
      (set `/Game/Afterlife/Core/BattleSystem/Enemies/BP_BaseEnemy.DropItemCount` 10 _returnvalue))))

(fn `UserConstructionScript`
  (`parent.UserConstructionScript`))
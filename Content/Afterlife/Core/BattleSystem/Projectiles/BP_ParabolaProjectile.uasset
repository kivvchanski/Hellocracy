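; Projectile actor for the battle system that launches toward a target position and damages the first actor it overlaps other than its DamageDealer.
; LaunchProjectile sets ProjectileMovement velocity to the offset to the target times Speed, so launch speed grows with distance.
; On overlap, DamageCollision sends TakeDamageMessage with damage, type, pushback, dealer and hit location, calls the empty CallEffect event, then destroys the projectile.
; Debug prints remain in both overlap branches.
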(event `LaunchProjectile`
  (params (TargetPosition :type "Vector Structure"))
  (set `MovementComponent.Velocity` (* (- TargetPosition (`self.K2_GetActorLocation`)) (`self.Speed`)) (`self.ProjectileMovement`)))

(event `self.DamageCollision.OnComponentBeginOverlap`
  (params (OverlappedComponent :type "PrimitiveComponent Object Reference") (OtherActor :type "Actor Object Reference") (OtherComp :type "PrimitiveComponent Object Reference") (OtherBodyIndex :type Integer) (bFromSweep :type Boolean) (SweepResult :type "HitResult Structure (by ref)"))
  (if (and (!= OtherActor (`self.DamageDealer`)) true)
    (`KismetSystemLibrary.PrintString` (`KismetSystemLibrary.GetObjectName` OtherActor))
    (message `/Game/Afterlife/Core/BattleSystem/BPI_Damagable.TakeDamage` OtherActor (`self.Damage`) (`self.DamageType`) (`self.PushingDistance`) (`self.DamageDealer`) (`self.K2_GetActorLocation`))
    (`self.CallEffect`)
    (`self.K2_DestroyActor`)
    (else
      (`KismetSystemLibrary.PrintString` "My Cords:")
      (`KismetSystemLibrary.PrintString` (`KismetStringLibrary.Concat_StrStr` (`KismetStringLibrary.Conv_VectorToString` (`self.K2_GetActorLocation`)))))))

(event `CallEffect`)

(fn `UserConstructionScript`)
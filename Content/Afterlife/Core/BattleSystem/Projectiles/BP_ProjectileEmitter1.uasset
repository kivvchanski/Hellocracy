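; Projectile emitter actor that repeatedly fires parabola projectiles at the first player's pawn.
; Tick runs through a DoOnce that resets after a two-second delay, pacing the shots.
; Each shot spawns a BP_ParabolaProjectile at the emitter's transform and launches it toward a point slightly above the pawn's location.
; A disconnected alternative using BP_MeshProjectile, arc-based LaunchToTarget and debug prints remains in the graph but never runs.
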(event `self.ReceiveTick`
  (params (DeltaSeconds :type "Float (single-precision)"))
  (bind (_returnvalue_x _returnvalue_y _returnvalue_z) (`KismetMathLibrary.BreakVector` (`self.K2_GetActorLocation` (`GameplayStatics.GetPlayerPawn` 0))))
  (`/Engine/EditorBlueprintResources/StandardMacros.DoOnce` false :!label _label
    (:`Completed`
      (bind _returnvalue (`|SpawnActorFromClass` "/Game/Afterlife/Core/BattleSystem/Projectiles/BP_ParabolaProjectile.BP_ParabolaProjectile_C" (`self.GetTransform`) "Undefined" "MultiplyWithRoot" null 0.0 "NewEnumerator0" 2.0 self null))
      (`/Game/Afterlife/Core/BattleSystem/Projectiles/BP_ParabolaProjectile.LaunchProjectile` _returnvalue (`KismetMathLibrary.MakeVector` _returnvalue_x _returnvalue_y (+ _returnvalue_z 100.0)))
      (`KismetSystemLibrary.Delay` 2.0)
      (goto _label :!via `Reset`))))

(fn `UserConstructionScript`)
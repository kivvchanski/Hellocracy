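; BP_BaseEnemy1 is an enemy character that registers with the GameState spawner and passes attack delay and patrol flag to its AI controller's Blackboard.
; AtackPlayer faces the player, damaging and pushing them if in range.
; TakeDamage updates health, plays an impact montage that pauses movement, launches the enemy away and reports damage to AI perception.
; Death drives a burnout dissolve through a shared Material Parameter Collection, then destroys the actor and randomly drops an item.
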(event `Init`
  (`KismetSystemLibrary.DelayUntilNextTick`)
  (bind _asbp_game_state (cast `/Game/Afterlife/Framework/BP_GameState` (`GameplayStatics.GetGameState`)))
  (`/Game/Afterlife/Core/BattleSystem/Enemies/Utils/BP_Spawner.AddSpawner` (`/Game/Afterlife/Framework/BP_GameState.Spawner` _asbp_game_state) (`self.GetTransform`) self))

(event `self.ReceiveBeginPlay`
  (bind _atackmontage (`self.AtackMontage`))
  (bind _returnvalue (`AIBlueprintHelperLibrary.GetAIController` self))
  (`self.Init`)
  (set `self.CurrentHP` (`self.MaxHP`))
  (bind _asaic_base_aicontroller (cast `/Game/Afterlife/Core/BattleSystem/Enemies/AIC_BaseAIController` _returnvalue))
  (set `/Game/Afterlife/Core/BattleSystem/Enemies/AIC_BaseAIController.PawnRef` self _asaic_base_aicontroller)
  (`/Engine/EditorBlueprintResources/StandardMacros.IsValid` _atackmontage
    (:`Is Valid`
      (set `self.AtackDelay` (+ (`AnimationAsset.GetPlayLength` _atackmontage) (`self.AddedDelay`))))
    (:`Is Not Valid`
      _))
  (`BlackboardComponent.SetValueAsFloat` (`AIBlueprintHelperLibrary.GetBlackboard` _returnvalue) "AtackDelay" (`self.AtackDelay`))
  (`BlackboardComponent.SetValueAsBool` (`AIBlueprintHelperLibrary.GetBlackboard` (`AIBlueprintHelperLibrary.GetAIController` self)) "MustPatrolling" (`self.MustPatroling`)))

(event `self.TakeDamage`
  (params (Damage :type "Float (double-precision)") (DamageType :type "/Game/Afterlife/Core/BattleSystem/E_DamageTypes Enum" :default "NewEnumerator0") (PushingDistance :type "Float (double-precision)") (DamageDealer :type "Actor Object Reference") (DamagePoint :type "Vector Structure"))
  (bind _returnvalue (`self.K2_GetActorLocation`))
  (bind _impactmontage (`self.ImpactMontage`))
  (bind _returnvalue_2 (* PushingDistance (- 1.0 0.0)))
  (bind _returnvalue_3 (`KismetMathLibrary.Normal` (- (`self.K2_GetActorLocation`) DamagePoint)))
  (`KismetSystemLibrary.PrintString` (`KismetStringLibrary.Conv_VectorToString` _returnvalue_3))
  (bind _output_get (set `self.CurrentHP` (- (`self.CurrentHP`) Damage)))
  (`self.OnHealthChanged` _output_get (`self.MaxHP`))
  (`|PlayMontage` (`self.Mesh`) (`self.ImpactMontage`) 1.0 0.0 "None" false
    (:`then`
      (`|ExecutionSequence`
        (:`then_0`
          (`/Engine/EditorBlueprintResources/StandardMacros.IsValid` _impactmontage
            (:`Is Valid`
              (bind _asaic_base_aicontroller (cast `/Game/Afterlife/Core/BattleSystem/Enemies/AIC_BaseAIController` (`AIBlueprintHelperLibrary.GetAIController` self)))
              (`/Game/Afterlife/Core/BattleSystem/Enemies/AIC_BaseAIController.DisableMovementForTime` _asaic_base_aicontroller (`AnimationAsset.GetPlayLength` _impactmontage)))))
        (:`then_1`
          (`self.LaunchCharacter` (`KismetMathLibrary.MakeVector` (* (.x _returnvalue_3) _returnvalue_2) (* (.y _returnvalue_3) _returnvalue_2) (* (.z _returnvalue_3) _returnvalue_2)) true)
          (`/Engine/EditorBlueprintResources/StandardMacros.IsValid` DamageDealer
            (:`Is Valid`
              (`AISense_Damage.ReportDamageEvent` (`AIBlueprintHelperLibrary.GetAIController` self) DamageDealer Damage))
            (:`Is Not Valid`
              _))
          (if (<= (`self.CurrentHP`) 0.0)
            (`self.OnEnemyDied`)
            (`KismetSystemLibrary.PrintString` "I m Die")
            (`GameplayStatics.PlaySoundAtLocation` (`self.DeathSound`) _returnvalue (struct) 2.0 1.0 0.0 null null null null)
            (`PrimitiveComponent.SetMaterial` (`self.Mesh`) 0 (`self.BurnOutMat`))
            (bind (_direction _newtrack_0) (`Timeline|Timeline`)
              (:`Update`
                (`KismetMaterialLibrary.SetScalarParameterValue` "/Game/Afterlife/Art/Characters/Materials/MPC_Burnout.MPC_Burnout" "TimeBurnOut" (`KismetMathLibrary.FClamp` (* _newtrack_0 0.5))))
              (:`Finished`
                (`self.K2_DestroyActor`)
                (if (<= (`KismetMathLibrary.RandomFloatInRange` 0.0 1.0) (`self.DropItemChance`))
                  ; WIP
                  (`|SpawnActorFromClass` (`self.DropItem`) (`KismetMathLibrary.Conv_VectorToTransform` _returnvalue) "Undefined" "MultiplyWithRoot" null (`self.DropItemCount`) (struct) null false null))))))))))

(event `AtackPlayer`
  (bind _returnvalue (>= (+ (`self.AtackRadius`) 50.0) (`self.GetDistanceTo` (`self.PlayerRef`) self)))
  (`self.K2_SetActorRotation` (`KismetMathLibrary.FindLookAtRotation` (`self.K2_GetActorLocation`) (`self.K2_GetActorLocation` (`self.PlayerRef`))))
  (if _returnvalue
    (message `/Game/Afterlife/Core/BattleSystem/BPI_Damagable.TakeDamage` (`self.PlayerRef`) (`self.Damage`) "NewEnumerator0" (`self.PushingDistance`) self (0.0 0.0 0.0))
    (`BlackboardComponent.SetValueAsBool` (`AIBlueprintHelperLibrary.GetBlackboard` (`AIBlueprintHelperLibrary.GetAIController` self)) "IsPlayerInAtackRadius" _returnvalue)))

(fn `UserConstructionScript`)
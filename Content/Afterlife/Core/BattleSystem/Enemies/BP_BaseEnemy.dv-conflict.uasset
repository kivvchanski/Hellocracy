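; Base enemy character for the battle system, handling health, player attacks, hit reactions and death.
; BeginPlay seeds the AI blackboard with patrol mode and a montage-based attack delay; attacks face the player and deal damage within range.
; Hits play an impact montage, pause AI movement, apply resistance-scaled knockback and report damage to AI.
; Death animates burnout through a shared Material Parameter Collection, then destroys the actor and rolls a work-in-progress item drop.
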(event `self.ReceiveBeginPlay`
  (bind _atackmontage (`self.AtackMontage`))
  (bind _returnvalue (`AIBlueprintHelperLibrary.GetAIController` self))
  (set `self.CurrentHP` (`self.MaxHP`))
  (bind _asaic_base_aicontroller (cast `/Game/Afterlife/Core/BattleSystem/Enemies/AIC_BaseAIController` _returnvalue))
  (set `/Game/Afterlife/Core/BattleSystem/Enemies/AIC_BaseAIController.PawnRef` self _asaic_base_aicontroller)
  (`/Engine/EditorBlueprintResources/StandardMacros.IsValid` _atackmontage
    (:`Is Valid`
      (set `self.AtackDelay` (+ (`AnimationAsset.GetPlayLength` _atackmontage) (`self.AddedDelay`))))
    (:`Is Not Valid`
      _))
  (`BlackboardComponent.SetValueAsFloat` (`AIBlueprintHelperLibrary.GetBlackboard` _returnvalue) "AtackDelay" (`self.AtackDelay`))
  (`BlackboardComponent.SetValueAsBool` (`AIBlueprintHelperLibrary.GetBlackboard` (`AIBlueprintHelperLibrary.GetAIController` self)) "MustPatrolling" (`self.MustPatroling`)))

(event `/Game/Afterlife/Core/BattleSystem/BPI_Damagable.TakeDamage`
  (params (Damage :type "Float (double-precision)") (DamageType :type "/Game/Afterlife/Core/BattleSystem/E_DamageTypes Enum" :default "NewEnumerator0") (PushingDistance :type "Float (double-precision)") (DamageDealer :type "Actor Object Reference") (DamagePoint :type "Vector Structure"))
  (bind (_returnvalue_x _returnvalue_y _returnvalue_z) (`KismetMathLibrary.BreakVector` (`self.GetActorForwardVector` DamageDealer)))
  (bind _returnvalue (`self.K2_GetActorLocation`))
  (bind _impactmontage (`self.ImpactMontage`))
  (bind _returnvalue_2 (* PushingDistance (- 1.0 (/ (`self.PushResistance`) 100.0))))
  (set `self.CurrentHP` (- (`self.CurrentHP`) Damage))
  (`|PlayMontage` (`self.Mesh`) (`self.ImpactMontage`) 1.0 0.0 "None" false
    (:`then`
      (`|ExecutionSequence`
        (:`then_0`
          (`/Engine/EditorBlueprintResources/StandardMacros.IsValid` _impactmontage
            (:`Is Valid`
              (bind _asaic_base_aicontroller (cast `/Game/Afterlife/Core/BattleSystem/Enemies/AIC_BaseAIController` (`AIBlueprintHelperLibrary.GetAIController` self)))
              (`/Game/Afterlife/Core/BattleSystem/Enemies/AIC_BaseAIController.DisableMovementForTime` _asaic_base_aicontroller (`AnimationAsset.GetPlayLength` _impactmontage)))))
        (:`then_1`
          (`self.LaunchCharacter` (`KismetMathLibrary.MakeVector` (* _returnvalue_x _returnvalue_2) (* _returnvalue_y _returnvalue_2) (* _returnvalue_z _returnvalue_2)) true)
          (`AISense_Damage.ReportDamageEvent` (`AIBlueprintHelperLibrary.GetAIController` self) DamageDealer Damage)
          (if (<= (`self.CurrentHP`) 0.0)
            (`GameplayStatics.PlaySoundAtLocation` (`self.DeathSound`) _returnvalue (struct) 2.0 1.0 0.0 null null null null)
            (`PrimitiveComponent.SetMaterial` (`self.Mesh`) 0 (`self.BurnOutMat`))
            (bind (_direction _newtrack_0) (`Timeline|Timeline`)
              (:`Update`
                (`KismetSystemLibrary.PrintString` "Time")
                (`KismetMaterialLibrary.SetScalarParameterValue` "/Game/Afterlife/Art/Characters/Materials/MPC_Burnout.MPC_Burnout" "TimeBurnOut" (`KismetMathLibrary.FClamp` (* _newtrack_0 0.5)))
                (bind _returnvalue_3 (`KismetMaterialLibrary.GetScalarParameterValue` "/Game/Afterlife/Art/Characters/Materials/MPC_Burnout.MPC_Burnout" "TimeBurnOut"))
                (`KismetSystemLibrary.PrintString` (`KismetStringLibrary.Conv_DoubleToString` _returnvalue_3)))
              (:`Finished`
                (`self.K2_DestroyActor`)
                (if (<= (`KismetMathLibrary.RandomFloatInRange` 0.0 1.0) (`self.DropItemChance`))
                  ; WIP
                  (`|SpawnActorFromClass` (`self.DropItem`) (`KismetMathLibrary.Conv_VectorToTransform` _returnvalue) "Undefined" "MultiplyWithRoot" null 10 null))))))))))

(event `AtackPlayer`
  (bind _returnvalue (>= (+ (`self.AtackRadius`) 50.0) (`self.GetDistanceTo` (`self.PlayerRef`) self)))
  (`self.K2_SetActorTransform` (`KismetAnimationLibrary.K2_LookAt` (`self.GetTransform`) (`self.K2_GetActorLocation` (`self.PlayerRef`)) (`SceneComponent.GetForwardVector` (`self.Mesh`))))
  (if _returnvalue
    (message `/Game/Afterlife/Core/BattleSystem/BPI_Damagable.TakeDamage` (`self.PlayerRef`) (`self.Damage`) "NewEnumerator0" 0.0 self (0.0 0.0 0.0))
    (`BlackboardComponent.SetValueAsBool` (`AIBlueprintHelperLibrary.GetBlackboard` (`AIBlueprintHelperLibrary.GetAIController` self)) "IsPlayerInAtackRadius" _returnvalue)))

(fn `UserConstructionScript`)
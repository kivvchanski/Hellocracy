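; BP_Spawner respawns enemies and items on the level at recorded transforms.
; AddSpawner and AddItemSpawner register each placed mob or item, mapping its transform to a class or item data and tracking the live instance.
; The Spawn event destroys all tracked mobs and items, then recreates them from those maps.
; Mobs take stats from class defaults, while items restore stored quantity and attach object.
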(event `Spawn`
  (bind _itemsonlevel (`self.ItemsOnLevel`))
  (for _array_element (`self.Mobs`)
    (`/Engine/EditorBlueprintResources/StandardMacros.IsValid` _array_element
      (:`Is Valid`
        (`self.K2_DestroyActor` _array_element))))
  (`KismetArrayLibrary.Array_Clear` (`self.Mobs`))
  (bind _keys (`BlueprintMapLibrary.Map_Keys` (`self.SpawnPoints`)))
  (for _array_element_2 _keys
    (bind _value (`BlueprintMapLibrary.Map_Find` (`self.SpawnPoints`) _array_element_2))
    (bind (_currenthp _pushresistance _maxhp _atackradius _playerref _atackdelay _damage _atackmontage _addeddelay _impactmontage _mustpatroling _dropitemchance _dropitem _pushingdistance _burnoutmat _deathsound _burnoutcollection _dropitemcount) (defaults `Object` _value))
    (bind _returnvalue (`|SpawnActorFromClass` _value _array_element_2 "Undefined" "MultiplyWithRoot" null _pushresistance _maxhp _atackradius _damage _dropitemcount null))
    (`KismetArrayLibrary.Array_Add` (`self.Mobs`) _returnvalue))
  (for _array_element_3 _itemsonlevel
    (`/Engine/EditorBlueprintResources/StandardMacros.IsValid` _array_element_3
      (:`Is Valid`
        (`self.K2_DestroyActor` _array_element_3))))
  (`KismetArrayLibrary.Array_Clear` _itemsonlevel)
  (bind _keys_2 (`BlueprintMapLibrary.Map_Keys` (`self.ItemSpawnPoints`)))
  (for _array_element_4 _keys_2
    (bind (_class _objecttoattach _quantity) (break `/Game/Afterlife/Core/BattleSystem/Enemies/Utils/F_LandingItems` (`BlueprintMapLibrary.Map_Find` (`self.ItemSpawnPoints`) _array_element_4)))
    (bind _returnvalue_2 (`|SpawnActorFromClass` _class _array_element_4 "Undefined" "MultiplyWithRoot" null _quantity (`.TableRowRef` (defaults `Object` _class)) _objecttoattach true null))
    (`KismetArrayLibrary.Array_Add` (`self.ItemsOnLevel`) _returnvalue_2)))

(fn `AddItemSpawner`
  (params (Transforms :type "Transform Structure") (ItemClass :type "/Game/Afterlife/Core/BattleSystem/Enemies/Utils/F_LandingItems Structure") (ItemRef :type "/Game/Afterlife/Core/Items/PickableItems/BP_BasePickableItem Object Reference"))
  (`BlueprintMapLibrary.Map_Add` (`self.ItemSpawnPoints`) Transforms ItemClass)
  (`KismetArrayLibrary.Array_Add` (`self.ItemsOnLevel`) ItemRef))

(fn `AddSpawner`
  (params (Position :type "Transform Structure") (Enemy :type "/Game/Afterlife/Core/BattleSystem/Enemies/BP_BaseEnemy Object Reference"))
  (`BlueprintMapLibrary.Map_Add` (`self.SpawnPoints`) Position (`GameplayStatics.GetObjectClass` Enemy))
  (`KismetArrayLibrary.Array_Add` (`self.Mobs`) Enemy))

(fn `UserConstructionScript`)
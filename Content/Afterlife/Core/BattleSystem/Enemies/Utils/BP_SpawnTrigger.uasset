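; BP_SpawnTrigger is a trigger volume that starts enemy spawning and restores the player to full HP when the main character enters it.
; One tick after BeginPlay it caches the Spawner reference from BP_GameState, with a debug print if valid.
; Each Box overlap by BP_MainCharacter calls Spawn on that spawner, then sets player 0's CurrentHP to MaxHP, with no one-shot guard.
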(event `self.ReceiveBeginPlay`
  (`KismetSystemLibrary.DelayUntilNextTick`)
  (bind _asbp_game_state (cast `/Game/Afterlife/Framework/BP_GameState` (`GameplayStatics.GetGameState`)))
  (bind _spawner (`/Game/Afterlife/Framework/BP_GameState.Spawner` _asbp_game_state))
  (set `self.SpawnerRef` _spawner)
  (`/Engine/EditorBlueprintResources/StandardMacros.IsValid` _spawner
    (:`Is Valid`
      (`KismetSystemLibrary.PrintString` "Spawner valid"))))

(event `self.Box.OnComponentBeginOverlap`
  (params (OverlappedComponent :type "PrimitiveComponent Object Reference") (OtherActor :type "Actor Object Reference") (OtherComp :type "PrimitiveComponent Object Reference") (OtherBodyIndex :type Integer) (bFromSweep :type Boolean) (SweepResult :type "HitResult Structure (by ref)"))
  (cast `/Game/Afterlife/Framework/Player/BP_MainCharacter` OtherActor)
  (`/Game/Afterlife/Core/BattleSystem/Enemies/Utils/BP_Spawner.Spawn` (`self.SpawnerRef`))
  (bind _asbp_main_character (cast `/Game/Afterlife/Framework/Player/BP_MainCharacter` (`GameplayStatics.GetPlayerPawn` 0)))
  (set `/Game/Afterlife/Framework/Player/BP_MainCharacter.CurrentHP` (`/Game/Afterlife/Framework/Player/BP_MainCharacter.MaxHP` _asbp_main_character) _asbp_main_character))

(fn `UserConstructionScript`)
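; BP_BaseEnemy_Toxic is the toxic enemy variant in the battle system, adding attack and hit feedback to inherited enemy behavior.
; AtackPlayer plays an attack sound and montage, deferring the parent's attack logic until a "Damage" montage notify begins.
; TakeDamage runs the parent's damage handling, then plays the toxic hit sound at the actor's location.
; Debug prints remain in the attack path.
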(event `self.AtackPlayer`
  (`KismetSystemLibrary.PrintString` (`KismetStringLibrary.Conv_DoubleToString` (`self.AtackDelay`)))
  (`GameplayStatics.PlaySoundAtLocation` "/Game/Afterlife/Sounds/Impacts/Toxic/CUE/Toxic_Attack_Cue.Toxic_Attack_Cue" (`self.K2_GetActorLocation`) (struct) 1.0 1.0 0.0 null null null null)
  (bind _notifyname (`|PlayMontage` (`self.Mesh`) (`self.AtackMontage`))
    (:`OnNotifyBegin`
      (if (== _notifyname "Damage")
        (`parent.AtackPlayer`)
        (`KismetSystemLibrary.PrintString` "I'm trying to atack")))))

(event `/Game/Afterlife/Core/BattleSystem/BPI_Damagable.TakeDamage`
  (params (Damage :type "Float (double-precision)") (DamageType :type "/Game/Afterlife/Core/BattleSystem/E_DamageTypes Enum" :default "NewEnumerator0") (PushingDistance :type "Float (double-precision)") (DamageDealer :type "Actor Object Reference") (DamagePoint :type "Vector Structure"))
  (`parent.TakeDamage` Damage DamageType PushingDistance DamageDealer DamagePoint)
  (`GameplayStatics.PlaySoundAtLocation` "/Game/Afterlife/Sounds/Impacts/Toxic/CUE/Toxic_Hit_Cue.Toxic_Hit_Cue" (`self.K2_GetActorLocation`) (struct) 1.0 1.0 0.0 null null null null))

(fn `UserConstructionScript`
  (`parent.UserConstructionScript`))
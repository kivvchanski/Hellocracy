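; BP_BaseEnemy_Toxic is the Toxic enemy in the battle system, a child enemy Blueprint that attacks the player in melee or at range.
; AtackPlayer picks by distance: within melee range it plays a montage whose "Damage" notify calls the parent attack, otherwise it calls RangeAtack.
; RangeAtack's notify turns it toward the player and launches a damaging parabola projectile slightly above them.
; Attack and hit sounds accompany these actions.
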(event `self.AtackPlayer`
  (if (<= (`self.GetDistanceTo` (`self.PlayerRef`) self) (`self.MeleeAtackDistance`))
    (`GameplayStatics.PlaySoundAtLocation` "/Game/Afterlife/Sounds/Impacts/Toxic/CUE/Toxic_Attack_Cue.Toxic_Attack_Cue" (`self.K2_GetActorLocation`) (struct) 1.0 1.0 0.0 null null null null)
    (bind _notifyname (`|PlayMontage` (`self.Mesh`) (`self.AtackMontage`))
      (:`OnNotifyBegin`
        (if (== _notifyname "Damage")
          (`parent.AtackPlayer`)
          (`KismetSystemLibrary.PrintString` "I'm trying to atack"))))
    (else
      (`self.RangeAtack`)
      (`KismetSystemLibrary.PrintString` "RangeAtack"))))

(event `RangeAtack`
  (bind (_returnvalue_x _returnvalue_y _returnvalue_z) (`KismetMathLibrary.BreakVector` (`self.K2_GetActorLocation` (`self.PlayerRef`))))
  (bind _notifyname (`|PlayMontage` (`self.Mesh`) (`self.RangeAtackMontage`))
    (:`OnNotifyBegin`
      (if (== _notifyname "Damage")
        (`self.K2_SetActorRotation` (`KismetMathLibrary.FindLookAtRotation` (`self.K2_GetActorLocation`) (`self.K2_GetActorLocation` (`self.PlayerRef`))))
        (bind _returnvalue (`|SpawnActorFromClass` "/Game/Afterlife/Core/BattleSystem/Projectiles/BP_ParabolaProjectile_Child.BP_ParabolaProjectile_Child_C" (`KismetMathLibrary.MakeTransform` (`SceneComponent.K2_GetComponentLocation` (`self.Scene`))) "Undefined" "MultiplyWithRoot" self (`self.RangeAtackDamage`) (`self.RangeAtackiType`) (`self.RangeAtackPushingDistance`) self null))
        (`/Game/Afterlife/Core/BattleSystem/Projectiles/BP_ParabolaProjectile.LaunchProjectile` _returnvalue (`KismetMathLibrary.MakeVector` _returnvalue_x _returnvalue_y (+ _returnvalue_z 150.0)))
        (`GameplayStatics.PlaySoundAtLocation` "/Game/Afterlife/Sounds/Impacts/Toxic/CUE/Toxic_Attack_Range_Cue.Toxic_Attack_Range_Cue" (`self.K2_GetActorLocation`) (struct) 1.0 1.0 0.0 null null null null)))))

(event `/Game/Afterlife/Core/BattleSystem/BPI_Damagable.TakeDamage`
  (params (Damage :type "Float (double-precision)") (DamageType :type "/Game/Afterlife/Core/BattleSystem/E_DamageTypes Enum" :default "NewEnumerator0") (PushingDistance :type "Float (double-precision)") (DamageDealer :type "Actor Object Reference") (DamagePoint :type "Vector Structure"))
  (`parent.TakeDamage` Damage DamageType PushingDistance DamageDealer DamagePoint)
  (`GameplayStatics.PlaySoundAtLocation` "/Game/Afterlife/Sounds/Impacts/Toxic/CUE/Toxic_Hit_Cue.Toxic_Hit_Cue" (`self.K2_GetActorLocation`) (struct) 1.0 1.0 0.0 null null null null))

(fn `UserConstructionScript`
  (`parent.UserConstructionScript`))
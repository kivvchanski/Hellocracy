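; Clerk enemy Blueprint that adds its own voice sounds and attack timing on top of inherited enemy combat behavior.
; Attacking stops the MediaSound component, plays the clerk attack cue attached to it and runs the attack montage, calling the parent attack only on the "Damage" notify.
; Taking damage runs the parent logic, then swaps to the hit cue if MediaSound is valid.
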(event `self.AtackPlayer`
  (bind _mediasound (`self.MediaSound`))
  (`SynthComponent.Stop` _mediasound)
  (`GameplayStatics.SpawnSoundAttached` "/Game/Afterlife/Sounds/Impacts/Clerk/CUE/Klerk_Attack_Cue.Klerk_Attack_Cue" _mediasound "None" (0.0 0.0 0.0) (struct) "KeepRelativeOffset" false 1.0 1.0 0.0 null null)
  (bind _notifyname (`|PlayMontage` (`self.Mesh`) (`self.AtackMontage`))
    (:`OnNotifyBegin`
      (if (== _notifyname "Damage")
        (`parent.AtackPlayer`)))))

(event `/Game/Afterlife/Core/BattleSystem/BPI_Damagable.TakeDamage`
  (params (Damage :type "Float (double-precision)") (DamageType :type "/Game/Afterlife/Core/BattleSystem/E_DamageTypes Enum" :default "NewEnumerator0") (PushingDistance :type "Float (double-precision)") (DamageDealer :type "Actor Object Reference") (DamagePoint :type "Vector Structure"))
  (bind _mediasound (`self.MediaSound`))
  (`parent.TakeDamage` Damage DamageType PushingDistance DamageDealer DamagePoint)
  (`/Engine/EditorBlueprintResources/StandardMacros.IsValid` _mediasound
    (:`Is Valid`
      (`SynthComponent.Stop` _mediasound)
      (`GameplayStatics.SpawnSoundAttached` "/Game/Afterlife/Sounds/Impacts/Clerk/CUE/Klerk_Hit_Cue.Klerk_Hit_Cue" _mediasound "None" (0.0 0.0 0.0) (struct) "KeepRelativeOffset" false 1.0 1.0 0.0 null null))))

(fn `UserConstructionScript`
  (`parent.UserConstructionScript`))
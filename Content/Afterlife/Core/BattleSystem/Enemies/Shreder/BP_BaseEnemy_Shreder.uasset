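; Shreder enemy that switches between melee and a ranged volley based on its distance to the player.
; Within melee distance, a montage notify triggers the parent attack; otherwise it fires a ranged attack behind a DoOnce.
; The volley turns to face the player on a notify and launches three projectiles, centered and offset to either side.
; After firing, attack radius shrinks to melee range for a cooldown, then restores.
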(event `self.ReceiveBeginPlay`
  (`parent.ReceiveBeginPlay`)
  (set `self.BaseAtackDistance` (`self.AtackRadius`)))

(event `self.AtackPlayer`
  (bind _mediasound (`self.MediaSound`))
  (if (<= (`self.GetDistanceTo` (`self.PlayerRef`) self) (`self.MeleeAtackDistance`))
    (`SynthComponent.Stop` _mediasound)
    (`GameplayStatics.SpawnSoundAttached` "/Game/Afterlife/Sounds/Impacts/Toxic/CUE/Toxic_Attack_Range_Cue.Toxic_Attack_Range_Cue" _mediasound "None" (0.0 0.0 0.0) (struct) "KeepRelativeOffset" false 1.0 1.0 0.0 null null)
    (bind _notifyname (`|PlayMontage` (`self.Mesh`) (`self.AtackMontage`))
      (:`OnNotifyBegin`
        (if (== _notifyname "Damage")
          (`parent.AtackPlayer`))))
    (else
      (`/Engine/EditorBlueprintResources/StandardMacros.DoOnce` false :!label _label
        (:`Completed`
          (`self.RangeAtack`)
          (set `self.AtackRadius` (`self.MeleeAtackDistance`))
          (`KismetSystemLibrary.Delay` 8.0)
          (set `self.AtackRadius` (`self.BaseAtackDistance`))
          (goto _label :!via `Reset`))))))

(event `/Game/Afterlife/Core/BattleSystem/BPI_Damagable.TakeDamage`
  (params (Damage :type "Float (double-precision)") (DamageType :type "/Game/Afterlife/Core/BattleSystem/E_DamageTypes Enum" :default "NewEnumerator0") (PushingDistance :type "Float (double-precision)") (DamageDealer :type "Actor Object Reference") (DamagePoint :type "Vector Structure"))
  (bind _mediasound (`self.MediaSound`))
  (`parent.TakeDamage` Damage DamageType PushingDistance DamageDealer DamagePoint)
  (`/Engine/EditorBlueprintResources/StandardMacros.IsValid` _mediasound
    (:`Is Valid`
      (`SynthComponent.Stop` _mediasound)
      (`GameplayStatics.SpawnSoundAttached` "/Game/Afterlife/Sounds/Impacts/Toxic/CUE/Toxic_Hit_Cue.Toxic_Hit_Cue" _mediasound "None" (0.0 0.0 0.0) (struct) "KeepRelativeOffset" false 1.0 1.0 0.0 null null))))

(event `RangeAtack`
  (bind (_returnvalue_x _returnvalue_y _returnvalue_z) (`KismetMathLibrary.BreakVector` (`self.K2_GetActorLocation` (`self.PlayerRef`))))
  (bind (_returnvalue_x_2 _returnvalue_y_2 _returnvalue_z_2) (`KismetMathLibrary.BreakVector` (`self.K2_GetActorLocation` (`self.PlayerRef`))))
  (bind (_returnvalue_x_3 _returnvalue_y_3 _returnvalue_z_3) (`KismetMathLibrary.BreakVector` (`self.K2_GetActorLocation` (`self.PlayerRef`))))
  (bind (_returnvalue_x_4 _returnvalue_y_4) (`KismetMathLibrary.BreakVector` (* (`SceneComponent.GetRightVector` (`self.CapsuleComponent`)) 200)))
  (bind (_returnvalue_x_5 _returnvalue_y_5) (`KismetMathLibrary.BreakVector` (* (`SceneComponent.GetRightVector` (`self.CapsuleComponent`)) -200)))
  (bind _notifyname (`|PlayMontage` (`self.Mesh`) (`self.RangeAtackMontage`))
    (:`OnNotifyBegin`
      (if (== _notifyname "Damage")
        (`KismetSystemLibrary.PrintString` "Damage")
        (`self.K2_SetActorRotation` (`KismetMathLibrary.FindLookAtRotation` (`self.K2_GetActorLocation`) (`self.K2_GetActorLocation` (`self.PlayerRef`))))
        (bind _returnvalue (`|SpawnActorFromClass` "/Game/Afterlife/Core/BattleSystem/Projectiles/BP_ShrederProjectile1.BP_ShrederProjectile1_C" (`KismetMathLibrary.MakeTransform` (`SceneComponent.K2_GetComponentLocation` (`self.Scene`))) "Undefined" "MultiplyWithRoot" self (`self.RangeAtackDamage`) (`self.RangeAtackiType`) (`self.RangeAtackPushingDistance`) self null))
        (`/Game/Afterlife/Core/BattleSystem/Projectiles/BP_ParabolaProjectile1.LaunchProjectile` _returnvalue (`KismetMathLibrary.MakeVector` _returnvalue_x_2 _returnvalue_y_2 (+ _returnvalue_z_2 150.0)))
        (`GameplayStatics.PlaySoundAtLocation` "/Game/Afterlife/Sounds/Impacts/Toxic/CUE/Toxic_Attack_Range_Cue.Toxic_Attack_Range_Cue" (`self.K2_GetActorLocation`) (struct) 1.0 1.0 0.0 null null null null)
        (bind _returnvalue_2 (`|SpawnActorFromClass` "/Game/Afterlife/Core/BattleSystem/Projectiles/BP_ShrederProjectile1.BP_ShrederProjectile1_C" (`KismetMathLibrary.MakeTransform` (`SceneComponent.K2_GetComponentLocation` (`self.Scene`))) "Undefined" "MultiplyWithRoot" self (`self.RangeAtackDamage`) (`self.RangeAtackiType`) (`self.RangeAtackPushingDistance`) self null))
        (`/Game/Afterlife/Core/BattleSystem/Projectiles/BP_ParabolaProjectile1.LaunchProjectile` _returnvalue_2 (`KismetMathLibrary.MakeVector` (+ _returnvalue_x_3 _returnvalue_x_5) (+ _returnvalue_y_3 _returnvalue_y_5) (+ _returnvalue_z_3 150.0)))
        (`GameplayStatics.PlaySoundAtLocation` "/Game/Afterlife/Sounds/Impacts/Toxic/CUE/Toxic_Attack_Range_Cue.Toxic_Attack_Range_Cue" (`self.K2_GetActorLocation`) (struct) 1.0 1.0 0.0 null null null null)
        (bind _returnvalue_3 (`|SpawnActorFromClass` "/Game/Afterlife/Core/BattleSystem/Projectiles/BP_ShrederProjectile1.BP_ShrederProjectile1_C" (`KismetMathLibrary.MakeTransform` (`SceneComponent.K2_GetComponentLocation` (`self.Scene`))) "Undefined" "MultiplyWithRoot" self (`self.RangeAtackDamage`) (`self.RangeAtackiType`) (`self.RangeAtackPushingDistance`) self null))
        (`/Game/Afterlife/Core/BattleSystem/Projectiles/BP_ParabolaProjectile1.LaunchProjectile` _returnvalue_3 (`KismetMathLibrary.MakeVector` (+ _returnvalue_x _returnvalue_x_4) (+ _returnvalue_y _returnvalue_y_4) (+ _returnvalue_z 150.0)))
        (`GameplayStatics.PlaySoundAtLocation` "/Game/Afterlife/Sounds/Impacts/Toxic/CUE/Toxic_Attack_Range_Cue.Toxic_Attack_Range_Cue" (`self.K2_GetActorLocation`) (struct) 1.0 1.0 0.0 null null null null)))))

(fn `UserConstructionScript`
  (`parent.UserConstructionScript`))
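; BP_QuestComponent is a quest component that checks whether its assigned quest can be completed.
; CheckQuest reads the quest's data table row and asks BP_GameInstance to find the first required item key.
; If the item is found, the game instance completes the quest by ID, and the function returns the search result.
; The check is marked WIP: it ignores other item keys and the interacting player, and prints the quest ID.
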(fn `CheckQuest`
  (params (InteractedPlayer :type "/Game/Afterlife/Framework/Player/BP_MainCharacter Object Reference"))
  (returns (Result :type Boolean))
  (bind (_quest_datatable _quest_rowname) (break `DataTableRowHandle` (`self.Quest`)))
  (bind _returnvalue (`|GetDataTableRow` _quest_datatable _quest_rowname)
    (:`then`
      (bind (_id _requiredquest _description _nextquestid _itemkeys) (break `/Game/Afterlife/Core/QuestSystem/F_QuestInstance` _returnvalue))
      (`KismetSystemLibrary.PrintString` (`KismetStringLibrary.Conv_NameToString` _id))
      (bind _asbp_game_instance (cast `/Game/Afterlife/Framework/BP_GameInstance` (`GameplayStatics.GetGameInstance`)))
      (bind _result (`/Game/Afterlife/Framework/BP_GameInstance.FindNeededItem` _asbp_game_instance (`|GetArrayItem` _itemkeys)))
      (if _result
        (`/Game/Afterlife/Framework/BP_GameInstance.CompleteQuest` _asbp_game_instance _id))
      (return _result))))
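; First-person player character that handles weapons, abilities, health, inventory and UI.
; Weapon swaps spawn a fresh actor and destroy the old one, also driving melee and the health-costing machine-gun burst.
; Stamina gates melee and capsule-traced teleport dash; grenade throws on G cost health and are blocked at critical HP.
; Damage drives a looping low-health material effect and ragdoll death, while a recurring camera trace updates crosshair friend/enemy state.
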(event `Key|Q`
  (params (Key :type "Key Structure"))
  ; Input Q
  (:`Pressed`
    (if (== (`self.SuperModeActivate`) false)
      (set `self.SuperModeActivate` true)
      (`/Game/Afterlife/Core/BattleSystem/BPI_Damagable.TakeDamage` 20.0)
      (set `self.RepeatCount` 50)
      (bind _returnvalue (`|SpawnActorFromClass` "/Game/Afterlife/Core/Items/Weapons/BP_Gun_MachineGun.BP_Gun_MachineGun_C" (`self.GetTransform`) "Undefined" "MultiplyWithRoot" null 10.0 50.0 self null))
      (`self.SwapWeapon` _returnvalue)
      (`self.PerformNextAction`))))

(event `PerformNextAction`
  ; Input Q
  (if (< (`self.CurrentAttackIndex`) (`self.RepeatCount`))
    (message `IMainAction.StartMainAction` (stale `Key|Q` _returnvalue))
    (set `self.CurrentAttackIndex` (+ (`self.CurrentAttackIndex`) 1))
    (`KismetSystemLibrary.Delay` 0.16)
    (`self.PerformNextAction`)
    (else
      (bind _returnvalue (`|SpawnActorFromClass` "/Game/Afterlife/Core/Items/Weapons/BP_Gun_Pistol.BP_Gun_Pistol_C" (`self.GetTransform`) "Undefined" "MultiplyWithRoot" null 30.0 1000.0 self null))
      (`self.SwapWeapon` _returnvalue)
      (set `self.SuperModeActivate` false)
      (set `self.CurrentAttackIndex` 0))))

(event `Key|G`
  (params (Key :type "Key Structure"))
  ; Input G
  (:`Pressed`
    (if (`self.CanGrenade`)
      (if (`self.bAbilityBlocked`)
        (`GameplayStatics.PlaySound2D` "/Game/Afterlife/Sounds/UI/WAV/UI_Error.UI_Error" 1.0 1.0 0.0 null null)
        (bind _returnvalue (`|CreateWidget` "/Game/Afterlife/UI/WBP_AbilityBlocked.WBP_AbilityBlocked_C"))
        (bind _output_get (set `self.WBP_AbilityBlock` _returnvalue))
        (`UserWidget.AddToViewport` _output_get 0)
        (else
          (set `self.CanGrenade` false)
          (`/Game/Afterlife/Core/BattleSystem/BPI_Damagable.TakeDamage` 10.0)
          (`IMainAction.StartMainAction` (`self.GrenadeRef`))
          (`KismetSystemLibrary.Delay` 1.5)
          (set `self.CanGrenade` true))))))

(event `Key|F`
  (params (Key :type "Key Structure"))
  ; INput F
  (:`Pressed`
    (if (`self.CanMelee`)
      (if (> (`StaminaComponent.GetCurrentStamina` (`self.StaminaComponent`)) (`self.MeleeStamina`))
        (set `self.CanMelee` false)
        (`StaminaComponent.ConsumeStamina` (`self.StaminaComponent`) (`self.MeleeStamina`))
        (`KismetSystemLibrary.Delay` 0.1)
        (bind _returnvalue (`|SpawnActorFromClass` "/Game/Afterlife/Core/Items/Weapons/BP_BaseMeleeWeaponNew.BP_BaseMeleeWeaponNew_C" (`self.GetTransform`) "Undefined" "MultiplyWithRoot" null 30.0 5000.0 self null))
        (`self.SwapWeapon` _returnvalue)
        (message `IMainAction.StartMainAction` _returnvalue)
        (`KismetSystemLibrary.Delay` 0.7)
        (bind _returnvalue_2 (`|SpawnActorFromClass` "/Game/Afterlife/Core/Items/Weapons/BP_Gun_Pistol.BP_Gun_Pistol_C" (`self.GetTransform`) "Undefined" "MultiplyWithRoot" null 30.0 1000.0 self null))
        (`self.SwapWeapon` _returnvalue_2)
        (set `self.CanMelee` true)
        (else
          (`GameplayStatics.PlaySound2D` "/Game/Afterlife/Sounds/UI/WAV/UI_Error.UI_Error" 1.0 1.0 0.0 null null))))))

(event `EnhancedInput|/Game/Afterlife/Framework/Player/IA_SwapItem`
  (params (ActionValue :type "Float (double-precision)") (ElapsedSeconds :type "Float (double-precision)") (TriggeredSeconds :type "Float (double-precision)") (InputAction :type "InputAction Object Reference" :default "/Game/Afterlife/Framework/Player/IA_SwapItem.IA_SwapItem"))
  (bind _inventorycomponent (`self.InventoryComponent`))
  (bind _inventorycomponent_2 (`self.InventoryComponent`))
  (bind _returnvalue (`InventoryComponent.GetSelectedSlot` _inventorycomponent_2))
  (bind _maxinvetoryslots (`InventoryComponent.MaxInvetorySlots` _inventorycomponent))
  (bind _output_item (break `InventorySlot` (`|GetArrayItem` (`InventoryComponent.InventorySlots` _inventorycomponent_2) _returnvalue)))
  (bind _returnvalue_2 (mod (`KismetMathLibrary.FTrunc` (+ (`InventoryComponent.GetSelectedSlot` _inventorycomponent) ActionValue)) _maxinvetoryslots))
  ; SwapItem
  (:`Triggered`
    (if (< _returnvalue_2 0)
      (`InventoryComponent.SelectSlot` (`self.InventoryComponent`) (+ _returnvalue_2 _maxinvetoryslots))
      (else
        (`InventoryComponent.SelectSlot` _inventorycomponent _returnvalue_2)))
    (`KismetSystemLibrary.PrintString` (`KismetStringLibrary.Concat_StrStr` "Select Item" (`KismetStringLibrary.Conv_IntToString` _returnvalue) (`KismetTextLibrary.Conv_TextToString` (`.DisplayName` (break `Item` _output_item)))))))

(event `Key|Two`
  (params (Key :type "Key Structure"))
  ; Input 2
  (:`Pressed`
    (bind _returnvalue (`|SpawnActorFromClass` "/Game/Afterlife/Core/Items/Weapons/BP_BaseMeleeWeaponNew.BP_BaseMeleeWeaponNew_C" (`self.GetTransform`) "Undefined" "MultiplyWithRoot" null 30.0 5000.0 self null))
    (`self.SwapWeapon` _returnvalue)))

(event `Key|One`
  (params (Key :type "Key Structure"))
  ; Input 1
  (:`Pressed`
    (bind _returnvalue (`|SpawnActorFromClass` "/Game/Afterlife/Core/Items/Weapons/BP_Gun_Pistol.BP_Gun_Pistol_C" (`self.GetTransform`) "Undefined" "MultiplyWithRoot" null 30.0 1000.0 self null))
    (set `self.Weapon` _returnvalue)
    (`self.SwapWeapon` _returnvalue)))

(event `EnhancedInput|/Game/Afterlife/Framework/Player/IA_Inventory`
  (params (ActionValue :type Boolean) (ElapsedSeconds :type "Float (double-precision)") (TriggeredSeconds :type "Float (double-precision)") (InputAction :type "InputAction Object Reference" :default "/Game/Afterlife/Framework/Player/IA_Inventory.IA_Inventory"))
  (bind _returnvalue (`GameplayStatics.GetPlayerController` 0))
  (bind _returnvalue_2 (`GameplayStatics.GetPlayerController` 0))
  (bind _activewidget (`self.ActiveWidget`))
  ; Inventory
  (:`Started`
    (`/Engine/EditorBlueprintResources/StandardMacros.IsValid` _activewidget
      (:`Is Valid`
        (`Widget.RemoveFromParent` _activewidget)
        (`GameplayStatics.SetGamePaused` false)
        (`WidgetBlueprintLibrary.SetInputMode_GameOnly` _returnvalue)
        (set `PlayerController.bShowMouseCursor` false _returnvalue)
        (set `self.ActiveWidget` null))
      (:`Is Not Valid`
        (bind _returnvalue_3 (`|CreateWidget` "/Game/Afterlife/UI/Inventory/WBP_Inventory.WBP_Inventory_C"))
        (set `self.ActiveWidget` _returnvalue_3)
        (`UserWidget.AddToViewport` _returnvalue_3 0)
        (set `PlayerController.bShowMouseCursor` true _returnvalue_2)
        (`WidgetBlueprintLibrary.SetInputMode_GameAndUIEx` _returnvalue_2 (`self.ActiveWidget`) "DoNotLock" false)
        (`GameplayStatics.SetGamePaused` true)))))

(event `Key|Four`
  (params (Key :type "Key Structure"))
  ; Input 4
  (:`Pressed`
    (bind _returnvalue (`|SpawnActorFromClass` "/Game/Afterlife/Core/Items/Weapons/BP_Gun_ShotGun.BP_Gun_ShotGun_C" (`self.GetTransform`) "Undefined" "MultiplyWithRoot" null 50.0 100.0 self null))
    (`self.SwapWeapon` _returnvalue)))

(event `Key|Three`
  (params (Key :type "Key Structure"))
  ; Input 3
  (:`Pressed`
    (`IMainAction.StartMainAction` (`self.GrenadeRef`))))

(event `Check If enemy`
  (bind _followcamera (`self.FollowCamera`))
  (bind _wbp_crosshair (`self.WBP_Crosshair`))
  (bind _returnvalue (`SceneComponent.K2_GetComponentLocation` _followcamera))
  ; Crosshair Color
  (bind (_outhit _returnvalue_2) (`KismetSystemLibrary.LineTraceSingle` _returnvalue (+ _returnvalue (* (`SceneComponent.GetForwardVector` _followcamera) (10000.0 10000.0 10000.0))) "TraceTypeQuery1"))
  (if _returnvalue_2
    (bind (_bblockinghit _binitialoverlap _time _distance _location _impactpoint _normal _impactnormal _physmat _hitactor) (`GameplayStatics.BreakHitResult` _outhit))
    (if (`self.ActorHasTag` _hitactor "Friendly")
      ;; Friendly
      (set `/Game/Afterlife/UI/Character_UI/WBP_Crosshair.IsFriendly?` true _wbp_crosshair)
      (set `/Game/Afterlife/UI/Character_UI/WBP_Crosshair.IsEnemy?` false _wbp_crosshair)
      (else
        ;; Enemy
        (set `/Game/Afterlife/UI/Character_UI/WBP_Crosshair.IsFriendly?` false _wbp_crosshair)
        (set `/Game/Afterlife/UI/Character_UI/WBP_Crosshair.IsEnemy?` false _wbp_crosshair)
        (if (`self.ActorHasTag` _hitactor "Enemy")
          ;; Enemy
          (set `/Game/Afterlife/UI/Character_UI/WBP_Crosshair.IsEnemy?` true _wbp_crosshair)))))
  (`KismetSystemLibrary.Delay` 0.001)
  (`self.Check If enemy`))

(event `OnPickUpUpdate`
  (bind _grenaderef (`self.GrenadeRef`))
  ; On Pick Up
  (`self.HideInteractionText`)
  (for _array_element (`InventoryComponent.InventorySlots` (`self.InventoryComponent`))
    (bind (_item _quantity) (break `InventorySlot` _array_element))
    (if (== "Grenade" (break `Item` _item))
      (set `/Game/Afterlife/Core/Items/Weapons/BP_Grenade.Count` (+ (`/Game/Afterlife/Core/Items/Weapons/BP_Grenade.Count` _grenaderef) _quantity) _grenaderef)))
  (set `TextBlock.Text` (`KismetTextLibrary.Conv_IntToText` (`/Game/Afterlife/Core/Items/Weapons/BP_Grenade.Count` (`self.GrenadeRef`))) (`/Game/Afterlife/UI/BaseTypes/WBP_ItemElem.TB_Count` (`/Game/Afterlife/UI/Character_UI/WBP_CharacterHUD.WBP_ItemElem_1` (`self.WidgetRef`))))
  (bind _asbp_base_gun_new (cast `/Game/Afterlife/Core/Items/Weapons/BP_BaseGunNew` (`self.ActiveWeapon`)))
  (`/Game/Afterlife/Core/Items/Weapons/BP_BaseGunNew.UpdateAmmoCount` _asbp_base_gun_new))

(event `Key|Five`
  (params (Key :type "Key Structure"))
  ; Input 5
  (:`Pressed`
    (bind _returnvalue (`|SpawnActorFromClass` "/Game/Afterlife/Core/Items/Weapons/BP_Gun_MachineGun.BP_Gun_MachineGun_C" (`self.GetTransform`) "Undefined" "MultiplyWithRoot" null 10.0 50.0 self null))
    (`self.SwapWeapon` _returnvalue)))

(event `Key|R`
  (params (Key :type "Key Structure"))
  ; Input R
)

(event `self.TakeDamage`
  (params (Damage :type "Float (double-precision)") (DamageType :type "/Game/Afterlife/Core/BattleSystem/E_DamageTypes Enum" :default "NewEnumerator0") (PushingDistance :type "Float (double-precision)") (DamageDealer :type "Actor Object Reference") (DamagePoint :type "Vector Structure"))
  ; Take Damage
  (`CharacterMovementComponent.AddImpulse` (`self.CharacterMovement`) (* (`KismetMathLibrary.Normal` (- (`self.K2_GetActorLocation`) DamagePoint)) PushingDistance) false)
  (bind _output_get (set `self.CurrentHP` (- (`self.CurrentHP`) Damage)))
  (`KismetSystemLibrary.PrintString` (`KismetStringLibrary.Conv_DoubleToString` _output_get))
  (`self.Damage HUD`)
  (bind _asplayer_controller (cast `PlayerController` (`self.GetController`)))
  (`PlayerController.ClientStartCameraShake` :`self` _asplayer_controller :`Shake` "/Game/Afterlife/Framework/Player/Camera_Shaking/BP_Camera_Hit_Shaker.BP_Camera_Hit_Shaker_C")
  (`GameplayStatics.PlaySound2D` "/Game/Afterlife/Sounds/Impacts/Player/Player_Hit_Cue.Player_Hit_Cue" 1.0 1.0 0.0 null null)
  (if (< (`self.CurrentHP`) 0.0)
    (`self.Death`)))

(event `TakeDamageinZone`
  (params (Damage :type "Float (double-precision)") (DamageType :type "/Game/Afterlife/Core/BattleSystem/E_DamageTypes Enum" :default "NewEnumerator0") (PushingDistance :type "Float (double-precision)") (DamageDealer :type "Actor Object Reference") (DamagePoint :type "Vector Structure"))
  ; Take Damage
  (`CharacterMovementComponent.AddImpulse` (`self.CharacterMovement`) (* (`KismetMathLibrary.Normal` (- (`self.K2_GetActorLocation`) DamagePoint)) PushingDistance) false)
  (bind _output_get (set `self.CurrentHP` (- (`self.CurrentHP`) Damage)))
  (`KismetSystemLibrary.PrintString` (`KismetStringLibrary.Conv_DoubleToString` _output_get))
  (cast `PlayerController` (`self.GetController`))
  (if (< (`self.CurrentHP`) 0.0)
    (`self.Death`)))

(event `EnhancedInput|/Game/Afterlife/Framework/Player/IA_PauseMenu`
  (params (ActionValue :type Boolean) (ElapsedSeconds :type "Float (double-precision)") (TriggeredSeconds :type "Float (double-precision)") (InputAction :type "InputAction Object Reference" :default "/Game/Afterlife/Framework/Player/IA_PauseMenu.IA_PauseMenu"))
  (bind _returnvalue (`GameplayStatics.GetPlayerController` 0))
  ; ЛОГИКА ПАУЗЫ (ПОМЕНЯТЬ ПРИ БИЛДЕ  НА ESC)
  (:`Started`
    (if (not (`self.IsPauseMenuOpened?`))
      (set `self.IsPauseMenuOpened?` true)
      (bind _returnvalue_2 (`|CreateWidget` "/Game/Afterlife/UI/Pause/WBP_Pause.WBP_Pause_C" _returnvalue))
      (bind _output_get (set `self.WBP_Pause` _returnvalue_2))
      (`UserWidget.AddToViewport` _output_get 0)
      (`WidgetBlueprintLibrary.SetInputMode_GameAndUIEx` _returnvalue (`self.WBP_Pause`) "LockOnCapture")
      (set `PlayerController.bShowMouseCursor` true (`GameplayStatics.GetPlayerController` 0))
      (`GameplayStatics.SetGamePaused` true)
      (else
        (set `self.IsPauseMenuOpened?` false)
        (`Widget.RemoveFromParent` (`self.WBP_Pause`))
        (`GameplayStatics.SetGamePaused` false)
        (`WidgetBlueprintLibrary.SetInputMode_GameOnly` _returnvalue)
        (set `PlayerController.bShowMouseCursor` false (`GameplayStatics.GetPlayerController` 0))))))

(event `Death`
  (bind _mesh (`self.Mesh`))
  ; Death Custom Event
  (set `self.IsDead` true)
  (`PrimitiveComponent.SetCollisionEnabled` _mesh "QueryAndPhysics")
  (`PrimitiveComponent.SetSimulatePhysics` _mesh true)
  (`SkeletalMeshComponent.SetPhysicsBlendWeight` _mesh 1.0)
  (`PrimitiveComponent.SetCollisionEnabled` (`self.CapsuleComponent`) "NoCollision")
  (`self.DisableInput` (`GameplayStatics.GetPlayerController` 0))
  (bind _returnvalue (`|CreateWidget` "/Game/Afterlife/UI/WBP_LoseMenu.WBP_LoseMenu_C"))
  (`UserWidget.AddToViewport` _returnvalue 0))

(event `self.OnJumped`
  ; Jump Camera Shake
  (bind _asplayer_controller (cast `PlayerController` (`self.GetController`)))
  (`PlayerController.ClientStartCameraShake` :`self` _asplayer_controller :`Shake` "/Game/Afterlife/Framework/Player/Camera_Shaking/BP_Camera_Jump_Shaker.BP_Camera_Jump_Shaker_C")
  (`GameplayStatics.PlaySound2D` "/Game/Afterlife/Sounds/Impacts/Player/Player_Jump_Cue.Player_Jump_Cue" 1.0 1.0 0.0 null null))

(event `Damage HUD`
  (bind _lowhealthaudio (`self.LowHealthAudio`))
  (bind _wbp_abilityblock (`self.WBP_AbilityBlock`))
  ; Damage HUD Custom Event
  (bind _output_get (set `self.Should Loop Effect ?` (<= (`self.CurrentHP`) 25.0)))
  (set `self.bAbilityBlocked` _output_get)
  (bind _play_rate (`self.Calculate Play Rate`))
  (`TimelineComponent.SetPlayRate` (`self.Damage Timeline`) _play_rate)
  (bind (_direction _damage_opacity) (`Timeline|Damage Timeline` :!label _label)
    (:`Update`
      (`MaterialInstanceDynamic.SetScalarParameterValue` (`self.Damage HUD Material`) "Opacity" _damage_opacity))
    (:`Finished`
      (switch `ETimelineDirection` _direction
        (:`Forward`
          ;; If alive -> reverse damage timeline
          (if (> (`self.CurrentHP`) 0.0)
            (`self.Reverse Damage HUD`)))
        (:`Backward`
          (if (`self.Should Loop Effect ?`)
            ;; If critical update effect and play again
            (`self.Update damage effect`)
            (`self.Damage HUD`)
            (`/Engine/EditorBlueprintResources/StandardMacros.DoOnce` false :!label _label_2
              (:`Completed`
                (bind _returnvalue (`GameplayStatics.SpawnSound2D` (`self.LowHealthSound`) 1.0 1.0 0.0 null))
                (set `self.LowHealthAudio` _returnvalue)))
            (else
              ;; If finished reverse update for next time
              (`/Engine/EditorBlueprintResources/StandardMacros.IsValid` _wbp_abilityblock
                (:`Is Valid`
                  (`Widget.RemoveFromParent` _wbp_abilityblock))
                (:`Is Not Valid`
                  _))
              (set `self.WBP_AbilityBlock` null)
              (`self.Update damage effect`)
              (`/Engine/EditorBlueprintResources/StandardMacros.IsValid` _lowhealthaudio
                (:`Is Valid`
                  (`AudioComponent.Stop` _returnvalue)
                  (`AudioComponent.Stop` _lowhealthaudio)
                  (`ActorComponent.K2_DestroyComponent` _lowhealthaudio)
                  (goto _label_2 :!via `Reset`))))))))))

(event `Reverse Damage HUD`
  ; Damage HUD Custom Event
  (goto _label :!via `Reverse`))

(event `Key|LeftControl`
  (params (Key :type "Key Structure"))
  ; Dash
  (:`Pressed`
    (if (`self.bCanDash`)
      (set `self.bCanDash` false)
      (`KismetSystemLibrary.K2_SetTimerDelegate` (delegate `ResetDash`) (`self.DashCooldown`))
      (if (> (`StaminaComponent.GetCurrentStamina` (`self.StaminaComponent`)) (`self.DashStamina`))
        (`StaminaComponent.ConsumeStamina` (`self.StaminaComponent`) (`self.DashStamina`))
        (if (> (`KismetMathLibrary.VSize` (`self.GetLastMovementInputVector`)) 0.1)
          (bind _location (`self.SafeDash` (`KismetMathLibrary.Normal` (`KismetMathLibrary.MakeVector` (.x (`KismetMathLibrary.Normal` (`self.GetLastMovementInputVector`))) (.y (`KismetMathLibrary.Normal` (`self.GetLastMovementInputVector`)))))))
          (`self.K2_SetActorLocation` _location)
          (`GameplayStatics.PlaySound2D` "/Game/Afterlife/Sounds/Impacts/Player/Player_Dash.Player_Dash" 1.0 1.0 0.0 null null)
          (bind _returnvalue (`|CreateWidget` "/Game/Afterlife/UI/WBP_Dash_CoolDown.WBP_Dash_CoolDown_C"))
          (bind _output_get (set `self.WBP_Dash_CD` _returnvalue))
          (`UserWidget.AddToViewport` _output_get 0)
          (`KismetSystemLibrary.Delay` 1.0)
          (`Widget.RemoveFromParent` (`self.WBP_Dash_CD`))
          (set `self.WBP_Dash_CD` null)
          (else
            (bind _location_2 (`self.SafeDash` (`KismetMathLibrary.GetForwardVector` (`KismetMathLibrary.MakeRotator` 0.0 0.0 (.yaw (`PlayerCameraManager.GetCameraRotation` (`GameplayStatics.GetPlayerCameraManager` 0)))))))
            (`self.K2_SetActorLocation` _location_2)
            (`GameplayStatics.PlaySound2D` "/Game/Afterlife/Sounds/Impacts/Player/Player_Dash.Player_Dash" 1.0 1.0 0.0 null null)
            (bind _returnvalue_2 (`|CreateWidget` "/Game/Afterlife/UI/WBP_Dash_CoolDown.WBP_Dash_CoolDown_C"))
            (bind _output_get_2 (set `self.WBP_Dash_CD` _returnvalue_2))
            (`UserWidget.AddToViewport` _output_get_2 0)
            (`KismetSystemLibrary.Delay` 1.0)
            (`Widget.RemoveFromParent` (`self.WBP_Dash_CD`))
            (set `self.WBP_Dash_CD` null)))
        (else
          (`GameplayStatics.PlaySound2D` "/Game/Afterlife/Sounds/UI/WAV/UI_Error.UI_Error" 1.0 1.0 0.0 null null))))))

(event `ResetDash`
  ; Dash
  (set `self.bCanDash` true))

(event `self.SwapWeapon`
  (params (NewWeapon :type "ABaseActiveItem Object Reference"))
  (bind _activeweapon (`self.ActiveWeapon`))
  ; Swap Weapon
  (`/Engine/EditorBlueprintResources/StandardMacros.IsValid` _activeweapon
    (:`Is Valid`
      (`self.K2_DestroyActor` _activeweapon))
    (:`Is Not Valid`
      _))
  (`parent.SwapWeapon` NewWeapon)
  (`/Engine/EditorBlueprintResources/StandardMacros.IsValid` NewWeapon
    (:`Is Valid`
      (`self.K2_AttachToComponent` NewWeapon (`self.Scene`) "None" "SnapToTarget" "SnapToTarget" "SnapToTarget" true)
      (bind _asbp_base_active_item (cast `/Game/Afterlife/Core/Items/BP_BaseActiveItem` NewWeapon))
      (`ABaseActiveItem.OnEquip` _asbp_base_active_item))))

(event `Key|H`
  (params (Key :type "Key Structure"))
  ; Input H
  (:`Pressed`
    (bind _returnvalue (`|GenericCreateObject` "/Game/Afterlife/Core/Items/Effects/BP_Heal.BP_Heal_C" 20.0))
    (`/Game/Afterlife/Core/Items/Effects/BP_BaseEffect.Use` _returnvalue self)))

(event `self.ReceiveBeginPlay`
  (bind _brush (`Image.Brush` (`/Game/Afterlife/UI/Character_UI/WBP_CharacterHUD.DamageHUD` (`self.WidgetRef`))))
  ; Begin Play
  (`|ExecutionSequence`
    (:`then_0`
      (`SceneComponent.K2_AttachToComponent` (`self.Mesh`) (`self.FollowCamera`) "None" "KeepWorld" "KeepWorld" "KeepWorld" true)
      (`|ExecutionSequence`
        (:`then_0`
          (bind _returnvalue (`|CreateWidget` "/Game/Afterlife/UI/Character_UI/WBP_CharacterHUD.WBP_CharacterHUD_C" (`GameplayStatics.GetPlayerController` 0)))
          (`UserWidget.AddToViewport` _returnvalue 0)
          (`/Game/Afterlife/UI/Character_UI/WBP_CharacterHUD.Init` _returnvalue self)
          (set `self.WidgetRef` _returnvalue)
          (bind _returnvalue_2 (`|SpawnActorFromClass` "/Game/Afterlife/Core/Items/Weapons/BP_Grenade.BP_Grenade_C" (`self.GetTransform`) "Undefined" "MultiplyWithRoot" null self null))
          (bind _output_get (set `self.GrenadeRef` _returnvalue_2))
          (set `/Game/Afterlife/Core/Items/Weapons/BP_Grenade.Count` 0 _output_get)
          (bind _returnvalue_3 (`|GetDataTableRow` "/Game/Afterlife/Core/Items/DT_Items.DT_Items" "Ammo_Stapler")
            (:`then`
              (`InventoryComponent.AddItem` (`self.InventoryComponent`) _returnvalue_3 20)
              (bind _returnvalue_4 (`|SpawnActorFromClass` "/Game/Afterlife/Core/Items/Weapons/BP_Gun_Pistol.BP_Gun_Pistol_C" (`KismetMathLibrary.MakeTransform` (.location (`self.GetTransform`)) (.rotation (`self.GetTransform`))) "Undefined" "MultiplyWithRoot" null 30.0 1000.0 self null))
              (set `self.Weapon` _returnvalue_4)
              (`self.SwapWeapon` _returnvalue_4)
              (bind _asbp_game_instance (cast `/Game/Afterlife/Framework/BP_GameInstance` (`GameplayStatics.GetGameInstance`)))
              (add `/Game/Afterlife/Framework/BP_GameInstance.OnQuestCompleted` _asbp_game_instance (delegate `QuestCompleted`))
              (`/Game/Afterlife/Framework/BP_GameInstance.GetFirstQuest` _asbp_game_instance)
              (`self.QuestCompleted` "None"))))
        (:`then_1`
          (bind _returnvalue_5 (`KismetMaterialLibrary.CreateDynamicMaterialInstance` (`WidgetBlueprintLibrary.GetBrushResourceAsMaterial` _brush)))
          (bind _output_get_2 (set `self.Damage HUD Material` _returnvalue_5))
          (`WidgetBlueprintLibrary.SetBrushResourceToMaterial` _brush _output_get_2))))
    (:`then_1`
      (bind _returnvalue_6 (`|CreateWidget` "/Game/Afterlife/UI/Character_UI/WBP_Crosshair.WBP_Crosshair_C"))
      (bind _output_get_3 (set `self.WBP_Crosshair` _returnvalue_6))
      (`UserWidget.AddToViewport` _output_get_3 0))
    (:`then_2`
      (`self.Check If enemy`))))

(event `QuestCompleted`
  (params (QuestID :type Name))
  ; Begin Play
  (`/Game/Afterlife/UI/Character_UI/WBP_CharacterHUD.UpdateQuests` (`self.WidgetRef`)))

(event `EnhancedInput|/Game/Afterlife/Framework/Player/IA_AltItemAction`
  (params (ActionValue :type Boolean) (ElapsedSeconds :type "Float (double-precision)") (TriggeredSeconds :type "Float (double-precision)") (InputAction :type "InputAction Object Reference" :default "/Game/Afterlife/Framework/Player/IA_AltItemAction.IA_AltItemAction"))
  (bind _weapon (`self.Weapon`))
  (:`Started`
    (`/Engine/EditorBlueprintResources/StandardMacros.IsValid` _weapon
      (:`Is Valid`
        (`IAlternateAction.StartAltAction` _weapon))))
  (:`Completed`
    (`/Engine/EditorBlueprintResources/StandardMacros.IsValid` _weapon
      (:`Is Valid`
        (`IAlternateAction.StopAltAction` _weapon)))))

(event `ChangeAmmoCount`
  (params (Current :type Integer) (Inventory :type Integer))
  ; Chage Ammo Count
  (set `TextBlock.Text` (`KismetTextLibrary.Conv_StringToText` (`KismetStringLibrary.Concat_StrStr` (`KismetStringLibrary.Conv_IntToString` Current) "/" (`KismetStringLibrary.Conv_IntToString` Inventory))) (`/Game/Afterlife/UI/Character_UI/WBP_CharacterHUD.AmmoCount` (`self.WidgetRef`))))

(event `EnhancedInput|/Game/Afterlife/Framework/Player/IA_MainItemAction`
  (params (ActionValue :type Boolean) (ElapsedSeconds :type "Float (double-precision)") (TriggeredSeconds :type "Float (double-precision)") (InputAction :type "InputAction Object Reference" :default "/Game/Afterlife/Framework/Player/IA_MainItemAction.IA_MainItemAction"))
  (bind _activeweapon (`self.ActiveWeapon`))
  ; Main Item Action
  (:`Triggered`
    (`/Engine/EditorBlueprintResources/StandardMacros.IsValid` _activeweapon
      (:`Is Valid`
        (`IMainAction.StartMainAction` _activeweapon))))
  (:`Canceled`
    (`/Engine/EditorBlueprintResources/StandardMacros.IsValid` _activeweapon :!label _label_3
      (:`Is Valid`
        (message `IMainAction.StopMainAction` _activeweapon))))
  (:`Completed`
    (goto _label_3)))

(event `AddInteractionText`
  (params (InteractionText :type String))
  ; Interaction Text
  (`/Game/Afterlife/UI/Character_UI/WBP_CharacterHUD.SetInteractText` (`self.WidgetRef`) InteractionText))

(event `EnhancedInput|/Game/Afterlife/Framework/Player/IA_Reload`
  (params (ActionValue :type Boolean) (ElapsedSeconds :type "Float (double-precision)") (TriggeredSeconds :type "Float (double-precision)") (InputAction :type "InputAction Object Reference" :default "/Game/Afterlife/Framework/Player/IA_Reload.IA_Reload"))
  ; Reload
  (:`Started`
    (message `/Game/Afterlife/Core/BattleSystem/BPI_Reloadable.Reload` (`self.ActiveWeapon`) 0)))

(event `HideInteractionText`
  ; Interaction Text
  (`/Game/Afterlife/UI/Character_UI/WBP_CharacterHUD.HideInteractText` (`self.WidgetRef`)))

(event `SetVisibleAmmo`
  ; Set Ammo
  (set `Widget.Visibility` "Visible" (`/Game/Afterlife/UI/Character_UI/WBP_CharacterHUD.AmmoCount` (`self.WidgetRef`))))

(event `SetInvisible`
  ; Set Ammo
  (set `Widget.Visibility` "Hidden" (`/Game/Afterlife/UI/Character_UI/WBP_CharacterHUD.AmmoCount` (`self.WidgetRef`))))

(event `PlayHandsAnim`
  (params (NewMontage :type "AnimMontage Object Reference"))
  (`|PlayMontage` (`self.Mesh`) NewMontage))

(fn `Calculate Play Rate`
  (returns (`Play Rate` :type "Float (double-precision)"))
  (bind _currenthp (`self.CurrentHP`))
  (if (<= _currenthp 25.0)
    (if (> _currenthp 0.0)
      (return (`self.Critical Play Rate`))
      (else
        (return (`KismetMathLibrary.MapRangeClamped` (`TimelineComponent.GetPlaybackPosition` (`self.Damage Timeline`)) 0.0 1.0 (`self.Max Death Play Rate`) 0.05))))
    (else
      (return (`self.Damage Play Rate`)))))

(fn `SafeDash`
  (params (Direction :type "Vector Structure"))
  (returns (Location :type "Vector Structure"))
  (bind _returnvalue (`self.K2_GetActorLocation`))
  (bind _returnvalue_2 (+ _returnvalue (* Direction (`self.DashDistancee`))))
  (bind (_outhit _returnvalue_3) (`KismetSystemLibrary.CapsuleTraceSingle` :`Start` _returnvalue :`End` _returnvalue_2 :`Radius` (`CapsuleComponent.GetUnscaledCapsuleSize` (`self.CapsuleComponent`)) :`HalfHeight` (`CapsuleComponent.GetUnscaledCapsuleHalfHeight` (`self.CapsuleComponent`)) :`TraceChannel` "TraceTypeQuery1" :`DrawDebugType` "ForOneFrame"))
  (if _returnvalue_3
    (return (`.Location` (`GameplayStatics.BreakHitResult` _outhit)))
    (else
      (return _returnvalue_2))))

(fn `Update damage effect`
  (bind _damage_hud_material (`self.Damage HUD Material`))
  (`MaterialInstanceDynamic.SetScalarParameterValue` _damage_hud_material "Random Offset" (`KismetMathLibrary.RandomFloatInRange` -2000.0 2000.0))
  (`MaterialInstanceDynamic.SetScalarParameterValue` _damage_hud_material "Noise Amount" (`KismetMathLibrary.MapRangeClamped` (`self.CurrentHP`) 100.0 0.0 1.0 5.0))
  (`MaterialInstanceDynamic.SetScalarParameterValue` _damage_hud_material "Contrast" (`KismetMathLibrary.MapRangeClamped` (`self.CurrentHP`) 100.0 0.0 7.0 0.5)))

(fn `UserConstructionScript`)
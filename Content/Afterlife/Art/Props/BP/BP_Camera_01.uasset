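; BP_Camera_01 is a camera prop that drives a 2D scene capture at a throttled rate.
; Ticking is off from BeginPlay until EnableCapture turns it on and takes an immediate capture with a debug print, and DisableCapture turns it off again.
; While ticking, a frame counter triggers CaptureScene once every UpdateFrequency frames, then resets, so the scene is not captured every frame.
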(event `self.ReceiveBeginPlay`
  (`self.SetActorTickEnabled` false :!label _label))

(event `Disable Capture`
  (goto _label))

(event `Enable Capture`
  (`self.SetActorTickEnabled` true)
  (`SceneCaptureComponent2D.CaptureScene` (`self.CaptureComponent2D`))
  (`KismetSystemLibrary.PrintString` "Capture Started!"))

(event `self.ReceiveTick`
  (params (DeltaSeconds :type "Float (single-precision)"))
  (bind _output_get (set `self.FrameCounter` (+ (`self.FrameCounter`) 1)))
  (if (== (mod _output_get (`self.Update Frequency`)) 0)
    (`SceneCaptureComponent2D.CaptureScene` (`self.CaptureComponent2D`))
    (set `self.FrameCounter` 0)))

(fn `UserConstructionScript`)
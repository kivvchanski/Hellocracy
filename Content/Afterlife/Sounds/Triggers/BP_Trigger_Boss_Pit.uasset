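; Boss pit trigger that starts a sound and shows a boss health bar when the player pawn first overlaps it.
; A DoOnce gates short delays, a 2D sound spawn and the creation of WBP_BossHealthBar, seeded with the monitored enemy's HP.
; It binds to that enemy's health-changed and died events, updating the bar on damage and, on death, removing it and stopping the sound.
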(event `OnEnemyDiedHandler`
  (`KismetSystemLibrary.PrintString` "I know")
  (`Widget.RemoveFromParent` (`self.HealthWidget`))
  (set `self.HealthWidget` null)
  (`KismetSystemLibrary.Delay` 0.2)
  (`AudioComponent.Stop` (stale `self.Trigger_0.OnComponentBeginOverlap` _returnvalue))
  (`KismetSystemLibrary.PrintString` "Stop"))

(event `self.Trigger_0.OnComponentBeginOverlap`
  (params (OverlappedComponent :type "PrimitiveComponent Object Reference") (OtherActor :type "Actor Object Reference") (OtherComp :type "PrimitiveComponent Object Reference") (OtherBodyIndex :type Integer) (bFromSweep :type Boolean) (SweepResult :type "HitResult Structure (by ref)"))
  (bind _enemytomonitor (`self.EnemyToMonitor`))
  (if (== OtherActor (`GameplayStatics.GetPlayerPawn` 0))
    (`/Engine/EditorBlueprintResources/StandardMacros.DoOnce` false
      (:`Completed`
        (`KismetSystemLibrary.PrintString` "Sound")
        (`KismetSystemLibrary.Delay` 0.2)
        (bind _returnvalue (`GameplayStatics.SpawnSound2D` (`self.SoundToPlay`) 1.0 1.0 0.0 null))
        (`KismetSystemLibrary.Delay` 0.2)
        (bind _returnvalue_2 (`|CreateWidget` "/Game/Afterlife/UI/WBP_BossHealthBar.WBP_BossHealthBar_C"))
        (`KismetSystemLibrary.PrintString` "Create")
        (bind _output_get (set `self.HealthWidget` _returnvalue_2))
        (`/Game/Afterlife/UI/WBP_BossHealthBar.UpdateHealth` _output_get (`/Game/Afterlife/Core/BattleSystem/Enemies/BP_BaseEnemy.CurrentHP` _enemytomonitor) (`/Game/Afterlife/Core/BattleSystem/Enemies/BP_BaseEnemy.MaxHP` _enemytomonitor))
        (`UserWidget.AddToViewport` _output_get 0)
        (`KismetSystemLibrary.PrintString` "add")
        (add `/Game/Afterlife/Core/BattleSystem/Enemies/BP_BaseEnemy.OnHealthChanged` _enemytomonitor (delegate `CustomEvent`))
        (add `/Game/Afterlife/Core/BattleSystem/Enemies/BP_BaseEnemy.OnEnemyDied` (`self.EnemyToMonitor`) (delegate `OnEnemyDiedHandler`))))))

(event `CustomEvent`
  (params (CurrentHP :type "Float (double-precision)") (MaxHP :type "Float (double-precision)"))
  (`/Game/Afterlife/UI/WBP_BossHealthBar.UpdateHealth` (stale `self.Trigger_0.OnComponentBeginOverlap` _output_get) CurrentHP MaxHP))

(event `self.Trigger_0.OnComponentEndOverlap`
  (params (OverlappedComponent :type "PrimitiveComponent Object Reference") (OtherActor :type "Actor Object Reference") (OtherComp :type "PrimitiveComponent Object Reference") (OtherBodyIndex :type Integer)))

(fn `UserConstructionScript`)
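; BP_Trigger_Sound_Main is a trigger volume that plays a one-time sound when something enters it.
; The first begin overlap of Trigger_0 passes a DoOnce, then plays SoundToPlay at the SoundEmitter location if the overlapping actor is the player pawn.
; Because DoOnce precedes the player check, another actor overlapping first consumes the trigger silently.
; End overlap is empty, and a BP_MainCharacter cast is left unconnected.
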(event `self.Trigger_0.OnComponentBeginOverlap`
  (params (OverlappedComponent :type "PrimitiveComponent Object Reference") (OtherActor :type "Actor Object Reference") (OtherComp :type "PrimitiveComponent Object Reference") (OtherBodyIndex :type Integer) (bFromSweep :type Boolean) (SweepResult :type "HitResult Structure (by ref)"))
  (`/Engine/EditorBlueprintResources/StandardMacros.DoOnce` false
    (:`Completed`
      (if (== OtherActor (`GameplayStatics.GetPlayerPawn` 0))
        (`GameplayStatics.PlaySoundAtLocation` (`self.SoundToPlay`) (`SceneComponent.K2_GetComponentLocation` (`self.SoundEmitter`)) (struct) 1.0 1.0 0.0 null null null null)))))

(event `self.Trigger_0.OnComponentEndOverlap`
  (params (OverlappedComponent :type "PrimitiveComponent Object Reference") (OtherActor :type "Actor Object Reference") (OtherComp :type "PrimitiveComponent Object Reference") (OtherBodyIndex :type Integer)))

(fn `UserConstructionScript`)
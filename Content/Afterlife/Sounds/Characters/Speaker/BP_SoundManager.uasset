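; BP_SoundManager is a manager Blueprint that plays random sounds from the SoundDT data table at a repeating interval.
; BeginPlay starts a looping timer set by IntervalSeconds, and each tick of that timer picks one random row.
; It then loops over every BP_Speaker in the level and calls PlaySound2D once per speaker with that row's sound, so playback is non-spatial.
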(event `OnTimer`
  (bind _sounddt (`self.SoundDT`))
  (bind _outactors (`GameplayStatics.GetAllActorsOfClass` "/Game/Afterlife/Sounds/Characters/Speaker/BP_Speaker.BP_Speaker_C"))
  (bind _outrownames (`DataTableFunctionLibrary.GetDataTableRowNames` _sounddt))
  (bind _returnvalue (`|GetDataTableRow` _sounddt (`|GetArrayItem` _outrownames (`KismetMathLibrary.RandomIntegerInRange` 0 (- (`KismetArrayLibrary.Array_Length` _outrownames) 1))))
    (:`then`
      (for _array_element _outactors
        (cast `/Game/Afterlife/Sounds/Characters/Speaker/BP_Speaker` _array_element)
        (`GameplayStatics.PlaySound2D` (`.Sound_2_B27E907E49DDA3163EB557BCBB223049` (break `/Game/Afterlife/Sounds/Characters/Speaker/ST_Speaker_Sound_Row` _returnvalue)) 1.0 1.0 0.0 null null)))))

(event `self.ReceiveBeginPlay`
  (`KismetSystemLibrary.K2_SetTimerDelegate` :`Time` (`self.IntervalSeconds`) :`bLooping` true))

(fn `UserConstructionScript`)